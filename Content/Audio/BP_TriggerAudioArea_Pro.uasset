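; One-shot audio trigger area that plays a sound when an actor with the player tag enters it.
; OnEnterTrigger asks the Audio Manager to play the configured sound ID with a probability and fade-in time.
; If UseEffect is set, it also applies an effect preset to that sound ID.
; The actor then destroys itself, so a player entry uses up the trigger even if the probability roll plays nothing.
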(event EventBeginPlay)

(event Collision|EventActorBeginOverlap
  (params (OtherActor :type Actor%20Object%20Reference)))

(event EventTick
  (params (DeltaSeconds :type Float%20%28single-precision%29)))

(event EventOnEnterTrigger
  (params (OverlappedComponent :type Primitive%20Component%20Object%20Reference) (OtherActor :type Actor%20Object%20Reference) (OtherComp :type Primitive%20Component%20Object%20Reference) (OtherBodyIndex :type Integer) (bFromSweep :type Boolean) (SweepResult :type Hit%20Result%20Structure%20%28by%20ref%29))
  (bind _returnvalue (Class|GlobalTagName|GetTagPlayer))
  (if (> (Utilities|Array|FindItem (Variables|/Script/Engine.Actor|GetTags OtherActor) _returnvalue) -1)
    (Class|AudioManager|PlaySoundwithProbability (Class|AudioManager|GetAudioManager) (Variables|Default|GetAudioID) (Variables|Default|GetProbability) 0 "0, 0, 0" (Variables|Default|GetFadeInTime) 0.0 1.0)
    (Utilities|FlowControl|Sequence
      (:then_0
        (if (Variables|Default|GetUseEffect)
          (Class|AudioManager|ApplyEffectPresetbySoundID (Class|AudioManager|GetAudioManager) (Variables|Default|GetAudioID) (Variables|Default|GetAudioEffectID))))
      (:then_1
        (Actor|DestroyActor)))))

(fn ConstructionScript)