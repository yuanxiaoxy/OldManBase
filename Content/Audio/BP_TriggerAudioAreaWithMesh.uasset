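; Audio trigger area with a static mesh that changes to a lit material while a player-tagged actor is inside.
; On trigger entry it saves the mesh's slot 0 material and applies LightMaterial; the AreaBox end overlap restores the saved material.
; Both events filter actors by the tag from GetTagPlayer.
; A Light timeline meant to drive the material's "Light" scalar parameter is present but never runs.
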(event OnComponentEndOverlap(AreaBox)
  (params (OverlappedComponent :type Primitive%20Component%20Object%20Reference) (OtherActor :type Actor%20Object%20Reference) (OtherComp :type Primitive%20Component%20Object%20Reference) (OtherBodyIndex :type Integer))
  (bind _returnvalue (Class|GlobalTagName|GetTagPlayer))
  (if (> (Utilities|Array|FindItem (Variables|/Script/Engine.Actor|GetTags OtherActor) _returnvalue) -1)
    (Rendering|Material|SetMaterial (Variables|Default|GetStaticMesh) 0 (Variables|Default|GetSourceMaterial))))

(event EventBeginPlay)

(event Collision|EventActorBeginOverlap
  (params (OtherActor :type Actor%20Object%20Reference)))

(event EventTick
  (params (DeltaSeconds :type Float%20%28single-precision%29)))

(event EventOnEnterTrigger
  (params (OverlappedComponent :type Primitive%20Component%20Object%20Reference) (OtherActor :type Actor%20Object%20Reference) (OtherComp :type Primitive%20Component%20Object%20Reference) (OtherBodyIndex :type Integer) (bFromSweep :type Boolean) (SweepResult :type Hit%20Result%20Structure%20%28by%20ref%29))
  (bind _staticmesh (Variables|Default|GetStaticMesh))
  (bind _returnvalue (Class|GlobalTagName|GetTagPlayer))
  (if (> (Utilities|Array|FindItem (Variables|/Script/Engine.Actor|GetTags OtherActor) _returnvalue) -1)
    (Variables|Default|SetSourceMaterial (Rendering|Material|GetMaterial _staticmesh 0))
    (Rendering|Material|SetMaterial _staticmesh 0 (Variables|Default|GetLightMaterial))))

(fn ConstructionScript)