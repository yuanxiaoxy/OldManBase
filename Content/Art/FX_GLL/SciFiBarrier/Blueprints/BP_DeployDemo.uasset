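; BP_DeployDemo is a demo actor for a sci-fi barrier deployment effect, driven through a material parameter.
; The construction script creates a dynamic instance of the barrier material on the static mesh.
; BeginPlay scales DeployTimeline's rate by deployment duration and applies any valid custom curve.
; Timeline updates feed DeploymentPercent, and its finish handler can loop after a delay, forward-only or ping-pong, though no graph node starts playback.
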(event EventBeginPlay
  (bind _deploytimeline (Variables|Default|GetDeployTimeline))
  (Components|Timeline|SetPlayRate _deploytimeline (/ 1.0 (* (Variables|Barrier|GetDeploymentDuration) 0.2)))
  (bind _curve (Variables|Barrier|GetCurve)
    (:then
      (Class|TimelineComponent|SetFloatCurve _deploytimeline _curve "Percent"))
    (:else)))

(event EventTick
  (params (DeltaSeconds :type Float%20%28single-precision%29)))

(fn ConstructionScript
  (bind _staticmeshcomponent (Variables|Debug|GetStaticMeshComponent))
  (bind _barriermaterial (Variables|Barrier|GetBarrierMaterial))
  (Rendering|Material|SetMaterial _staticmeshcomponent 0 _barriermaterial)
  (bind _returnvalue (Rendering|Material|CreateDynamicMaterialInstance _staticmeshcomponent 0 _barriermaterial "None" :!class /Script/Engine.PrimitiveComponent))
  (Variables|Barrier|SetDyMat _returnvalue))