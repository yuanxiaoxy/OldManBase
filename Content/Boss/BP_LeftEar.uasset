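; Left ear of the boss head, a draggable part that feeds drag progress to BossHead while the player works its cable.
; Drag start enables Tick, turns on the ear light and raises post-process light strength; drag stop disables Tick, fades the effect and switches the light off after a short delay.
; Tick adds clamped, speed-scaled progress only while TargetCable has a player and its movement direction matches TargetForward.
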(event Custom|自定义事件
  (params (TimerId :type String))
  (Default|SetLeftEarLightFalse (Variables|Default|GetBossHead)))

(event EventBeginPlay)

(event Collision|EventActorBeginOverlap
  (params (OtherActor :type Actor%20Object%20Reference)))

(event EventTick
  (params (DeltaSeconds :type Float%20%28single-precision%29))
  (if (Variables|Default|GetTargetForward)
    (if (and (Variables|/Game/Boss/BP_BossCable.BP_BossCable_C|GetMoveForward (Variables|Default|GetTargetCable)) (and (Variables|Default|GetIsDraged) (Variables|/Game/Boss/BP_BossCable.BP_BossCable_C|GetHasPlayer (Variables|Default|GetTargetCable))))
      (Class|OldManBossHead|LeftEarDragedAdd (Variables|Default|GetBossHead) (Math|Float|Clamp(Float) (* DeltaSeconds (Variables|Default|GetMoveSpeed))) :!label _label)
      (Development|PrintString (Utilities|String|ToString(Rotator) (Transformation|GetActorRotation (Variables|Default|GetBossHead)))))
    (elif (and (not (Variables|/Game/Boss/BP_BossCable.BP_BossCable_C|GetMoveForward (Variables|Default|GetTargetCable))) (and (Variables|Default|GetIsDraged) (Variables|/Game/Boss/BP_BossCable.BP_BossCable_C|GetHasPlayer (Variables|Default|GetTargetCable))))
      (goto _label))))

(event EventOnStartDragging
  (Variables|Default|SetIsDraged true)
  (Actor|Tick|SetActorTickEnabled true)
  (Default|SetLeftEarLightTrue (Variables|Default|GetBossHead))
  (Class|PostProcessManager|SetLightStrength (Class|PostProcessManager|GetPostProcessManager) 15.0))

(event EventOnStopDragging
  (Variables|Default|SetIsDraged false)
  (Actor|Tick|SetActorTickEnabled false)
  (Class|PostProcessManager|Fade2None (Class|PostProcessManager|GetPostProcessManager))
  (Class|MonoManager|SetTimeout (Class|MonoManager|GetMonoManager) 0.5 (delegate Custom|自定义事件)))

(fn ConstructionScript)