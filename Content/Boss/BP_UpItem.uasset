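; BP_UpItem is a Boss-folder helper that moves a referenced MoveActor from its starting position to TargetPos.
; BeginPlay caches the start position and calls Upitem immediately if IsStartUp is set.
; Upitem snaps the actor to the target through a lerp fixed at full alpha, printing the position.
; A timeline meant to drive the move and fire CallOnUpItemCompelete is unconnected, so neither animation nor completion callback runs.
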(event Custom|Upitem
  (bind _targetpos (Variables|Default|GetTargetPos))
  (bind _initpos (Variables|Default|GetInitPos))
  (bind _returnvalue (Math|Vector|Lerp(Vector) _initpos _targetpos 1.0))
  (Transformation|SetActorLocation (Variables|Default|GetMoveActor) _returnvalue false false)
  (Development|PrintText (Utilities|Text|ToText(String) _returnvalue)))

(event EventBeginPlay
  (bind _moveactor (Variables|Default|GetMoveActor))
  (bind _returnvalue (Transformation|GetActorLocation _moveactor))
  (Transformation|SetActorLocation _moveactor _returnvalue false false)
  (Variables|Default|SetInitPos _returnvalue)
  (if (Variables|Default|GetIsStartUp)
    (CallFunction|Upitem)))

(fn ConstructionScript)