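; Boss-area trigger that plays an alarm sequence and then opens the third door when the player first overlaps it.
; On entry it changes the door's monitor material, plays a warning sound and starts a repeating timer that toggles post-process saturation, contrast and gamma to flash the screen.
; Audio-manager finished callbacks chain a second alarm sound, then stop the blink, restore the initial color grading and open the door.
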(event Custom|Blink
  (bind _baohe (Variables|Default|GetBaohe))
  (bind _duibi (Variables|Default|GetDuiBi))
  (bind _gama (Variables|Default|GetGaMa))
  (bind _baohe_init (Variables|Default|GetBaohe_Init))
  (bind _duibi_init (Variables|Default|GetDuiBi_Init))
  (bind _gama_init (Variables|Default|GetGaMa_Init))
  (if (Variables|Default|GetIsA)
    (Variables|Default|SetIsA false)
    (Utilities|Struct|SetmembersinPostProcessSettings (Variables|/Script/Engine.PostProcessVolume|GetSettings (Variables|Default|GetPostProcessVolum)) (Math|Vector4|MakeVector4 (.x _baohe) (.y _baohe) (.z _baohe) 1.0) (Math|Vector4|MakeVector4 (.x _duibi) (.y _duibi) (.z _duibi) 1.0) (Math|Vector4|MakeVector4 (.x _gama) (.y _gama) (.z _gama) 1.0))
    (else
      (Variables|Default|SetIsA true)
      (Utilities|Struct|SetmembersinPostProcessSettings (Variables|/Script/Engine.PostProcessVolume|GetSettings (Variables|Default|GetPostProcessVolum)) (Math|Vector4|MakeVector4 (.x _baohe_init) (.y _baohe_init) (.z _baohe_init) 1.0) (Math|Vector4|MakeVector4 (.x _duibi_init) (.y _duibi_init) (.z _duibi_init) 1.0) (Math|Vector4|MakeVector4 (.x _gama_init) (.y _gama_init) (.z _gama_init) 1.0)))))

(event Custom|ThirdDoor
  (params (SoundID :type Name))
  (EventDispatchers|UnbindEventfromOnSoundFinished (Class|AudioManager|GetAudioManager) (delegate Custom|ThirdDoor))
  (EventDispatchers|BindEventtoOnSoundFinished (Class|AudioManager|GetAudioManager) (delegate Custom|ThirdDoorr))
  (Class|AudioManager|PlaySound (Class|AudioManager|GetAudioManager) "Boss_AlermFace" self "0, 0, 0" 0.0 0.0 1.0))

(event Custom|ThirdDoorr
  (params (SoundID :type Name))
  (bind _baohe_init (Variables|Default|GetBaohe_Init))
  (bind _duibi_init (Variables|Default|GetDuiBi_Init))
  (bind _gama_init (Variables|Default|GetGaMa_Init))
  (EventDispatchers|UnbindEventfromOnSoundFinished (Class|AudioManager|GetAudioManager) (delegate Custom|ThirdDoorr))
  (Class|MonoManager|ClearTimer (Class|MonoManager|GetMonoManager) "Boss_Blink")
  (Utilities|Struct|SetmembersinPostProcessSettings (Variables|/Script/Engine.PostProcessVolume|GetSettings (Variables|Default|GetPostProcessVolum)) (Math|Vector4|MakeVector4 (.x _baohe_init) (.y _baohe_init) (.z _baohe_init) 1.0) (Math|Vector4|MakeVector4 (.x _duibi_init) (.y _duibi_init) (.z _duibi_init) 1.0) (Math|Vector4|MakeVector4 (.x _gama_init) (.y _gama_init) (.z _gama_init) 1.0))
  (Default|OpenDoor (Variables|Default|GetDoor)))

(event EventBeginPlay)

(event Collision|EventActorBeginOverlap
  (params (OtherActor :type Actor%20Object%20Reference))
  (if (Variables|Default|GetisFirst)
    (Variables|Default|SetisFirst false)
    (bind _returnvalue (Class|GlobalTagName|GetTagPlayer))
    (if (> (Utilities|Array|FindItem (Variables|/Script/Engine.Actor|GetTags OtherActor) _returnvalue) -1)
      (EventDispatchers|BindEventtoOnSoundFinished (Class|AudioManager|GetAudioManager) (delegate Custom|ThirdDoor))
      (Class|AudioManager|PlaySound (Class|AudioManager|GetAudioManager) "Boss_WarningAlerm" self "0, 0, 0" 0.0 0.0 1.0)
      (Rendering|Material|SetMaterial (Variables|/Game/BluePrints/Item/BossDoor/BP_BossDoorDrag.BP_BossDoorDrag_C|GetSM_UpDoor (Variables|Default|GetDoor)) 1 "/Game/Art/boss/door/MI_Monitor_02_03.MI_Monitor_02_03")
      (Class|MonoManager|SetIntervalSimplewithId (Class|MonoManager|GetMonoManager) 0.5 "Boss_Blink" (delegate Custom|Blink)))))

(event EventTick
  (params (DeltaSeconds :type Float%20%28single-precision%29)))

(fn ConstructionScript)