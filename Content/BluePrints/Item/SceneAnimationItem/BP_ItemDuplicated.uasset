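; Scene animation item that moves a configurable static mesh, set in the construction script, along a referenced spline actor.
; MoveItem picks a looping or one-shot timeline from Loop, scales its rate by Time, and plays it forward or reversed.
; Each update places the actor by spline distance, adding a curve-driven height offset that samples a constant zero in loop mode.
; Rotation follows the spline, optional only when looping via CanChangeRotation.
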(event Custom|MoveItem
  (bind _splinetofollow (Variables|Default|GetSplineToFollow))
  (bind _splinetofollow_2 (Variables|Default|GetSplineToFollow))
  (bind _splinetofollow_3 (Variables|Default|GetSplineToFollow))
  (bind _spline (Variables|/Game/BluePrints/Item/SceneAnimationItem/BP_ItemSpline.BP_ItemSpline_C|GetSpline _splinetofollow))
  (bind _spline_2 (Variables|/Game/BluePrints/Item/SceneAnimationItem/BP_ItemSpline.BP_ItemSpline_C|GetSpline _splinetofollow_2))
  (bind _spline_3 (Variables|/Game/BluePrints/Item/SceneAnimationItem/BP_ItemSpline.BP_ItemSpline_C|GetSpline _splinetofollow_3))
  (if (Variables|Default|GetLoop)
    (Components|Timeline|SetPlayRate (Variables|Default|Get时间轴_0) (/ 1.0 (Variables|Default|GetTime)))
    (if (Variables|Default|GetReserveStart)
      (bind _movetrack (Timeline|时间轴_0 ReverseFromEnd)
        (:Update
          (if (Variables|Default|GetCanChangeRotation)
            (Variables|Default|SetRotation (Spline|GetRotationatDistanceAlongSpline _spline_3 (Math|Float|Lerp 0.0 (Spline|GetSplineLength _spline_3) _movetrack) "World"))
            (else
              (Variables|Default|SetRotation (Transformation|GetActorRotation))))
          (Transformation|SetActorLocationAndRotation (Math|Vector|MakeVector (.x (Spline|GetLocationatDistanceAlongSpline _spline_2 (Math|Float|Lerp 0.0 (Spline|GetSplineLength _spline_2) _movetrack) "World")) (.y (Spline|GetLocationatDistanceAlongSpline _spline_2 (Math|Float|Lerp 0.0 (Spline|GetSplineLength _spline_2) _movetrack) "World")) (+ (.z (Spline|GetLocationatDistanceAlongSpline _spline_2 (Math|Float|Lerp 0.0 (Spline|GetSplineLength _spline_2) _movetrack) "World")) (* (Variables|Default|GetFloatExtremum) (Math|Curves|GetFloatValue (Variables|Default|GetFloatCurve) (Math|Float|%(Float) (* 0.0 (Variables|Default|GetFloatRate)) 1.0))))) (Variables|Default|GetRotation))))
      (else
        (Timeline|时间轴_0 PlayFromStart)))
    (else
      (Components|Timeline|SetPlayRate (Variables|Default|Get时间轴) (/ 1.0 (Variables|Default|GetTime)))
      (if (Variables|Default|GetReserveStart)
        (bind _movetrack_2 (Timeline|时间轴 ReverseFromEnd)
          (:Update
            (Transformation|SetActorLocationAndRotation (Math|Vector|MakeVector (.x (Spline|GetLocationatDistanceAlongSpline _spline (Math|Float|Lerp 0.0 (Spline|GetSplineLength _spline) _movetrack_2) "World")) (.y (Spline|GetLocationatDistanceAlongSpline _spline (Math|Float|Lerp 0.0 (Spline|GetSplineLength _spline) _movetrack_2) "World")) (+ (.z (Spline|GetLocationatDistanceAlongSpline _spline (Math|Float|Lerp 0.0 (Spline|GetSplineLength _spline) _movetrack_2) "World")) (* (Variables|Default|GetFloatExtremum) (Math|Curves|GetFloatValue (Variables|Default|GetFloatCurve) (Math|Float|%(Float) (* _movetrack_2 (Variables|Default|GetFloatRate)) 1.0))))) (Spline|GetRotationatDistanceAlongSpline _spline (Math|Float|Lerp 0.0 (Spline|GetSplineLength _spline) _movetrack_2) "World"))))
        (else
          (Timeline|时间轴 PlayFromStart))))))

(fn ConstructionScript
  (Components|StaticMesh|SetStaticMesh (Variables|Default|GetItem_0) (Variables|Default|GetItemMesh)))