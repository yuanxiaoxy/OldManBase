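; BP_EnemyGenerateArea is a trigger area that turns approach-enemy generation on or off when the player enters it.
; On overlap with an actor tagged tag_Player, its StartOrEnd flag selects the action.
; A start area passes its spawn interval, move speed and spawn distance to the Enemy Manager, then starts the approach enemy generator; an end area stops it.
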(event EventBeginPlay)

(event Collision|EventActorBeginOverlap
  (params (OtherActor :type Actor%20Object%20Reference))
  (bind _returnvalue (Class|OldManEnemyManager|GetEnemyManager))
  (if (> (Utilities|Array|FindItem (Variables|/Script/Engine.Actor|GetTags OtherActor) "tag_Player") -1)
    (if (Variables|Default|GetStartOrEnd)
      (Class|OldManEnemyManager|UpdateApproachEnemySettings _returnvalue (Variables|Default|GetEnemy%20Spawn%20Interval) (Variables|Default|GetEnemy%20Move%20Speed) (Variables|Default|GetEnemy%20Spawn%20Distance))
      (Class|OldManEnemyManager|StartApproachEnemyGenerator _returnvalue)
      (else
        (Class|OldManEnemyManager|StopApproachEnemyGenerator _returnvalue)))))

(event EventTick
  (params (DeltaSeconds :type Float%20%28single-precision%29)))

(fn ConstructionScript)