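; BP_ManagerAgent is a setup actor that configures and starts the game's enemy manager singleton.
; On BeginPlay it fetches the manager and passes it its own pool count, spawn interval and enemy info, plus BP_AdEnemyCharacter as the enemy class.
; It then calls InitializeSingleton, acting as a Blueprint-side bridge for the manager's settings with no other active logic.
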(event EventBeginPlay
  (bind _output_get (Variables|Default|SetEnemyManager (Class|OldManEnemyManager|GetEnemyManager)))
  (Variables|/Script/OldManEnemy.OldManEnemyManager|SetObjectPoolCount _output_get (Variables|Default|GetObjectPoolCount))
  (Variables|/Script/OldManEnemy.OldManEnemyManager|SetEnemyBlueprintClass _output_get "/Game/Enemy/BP_AdEnemyCharacter.BP_AdEnemyCharacter_C")
  (Variables|/Script/OldManEnemy.OldManEnemyManager|SetSpawnInterval _output_get (Variables|Default|GetSpawnInterval))
  (Variables|/Script/OldManEnemy.OldManEnemyManager|SetEnemyInfos _output_get (Variables|Default|GetBP_EnemyInfos))
  (Class|OldManEnemyManager|InitializeSingleton (Variables|Default|GetEnemyManager)))

(event Collision|EventActorBeginOverlap
  (params (OtherActor :type Actor%20Object%20Reference)))

(event EventTick
  (params (DeltaSeconds :type Float%20%28single-precision%29)))

(fn ConstructionScript)