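; BP_ItemManager spawns a staggered stream of animated items that move along a spline, using a referenced Item as the template.
; On BeginPlay it starts the template moving, then a delayed loop spawns Number copies at IntervalTime spacing at the spline's first point.
; Each copy inherits the template's spline, mesh, float, loop and timing settings, passes its FloatCurve to MoveTimeLine, then calls MoveItem.
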(event EventBeginPlay
  (bind _item (Variables|Default|GetItem))
  (Default|MoveItem (Variables|Default|GetItem))
  (Utilities|ForLoopwithDelayFirst 0 (- (Variables|Default|GetNumber) 1) (Variables|Default|GetIntervalTime)
    (:LoopBody
      (bind _returnvalue (Game|SpawnActorfromClass (Utilities|GetClass (Variables|Default|GetItem)) (Math|Conversions|ToTransform(Vector) (Spline|GetLocationatSplinePoint (Variables|/Game/BluePrints/Item/SceneAnimationItem/OldMan_Spline/BP_ItemSpline.BP_ItemSpline_C|GetSpline (Variables|/Game/BluePrints/Item/SceneAnimationItem/OldMan_Spline/BP_Item.BP_Item_C|GetSplineToFollow _item)) 0 "World")) "Undefined" "MultiplyWithRoot" 0 0))
      (Variables|/Game/BluePrints/Item/SceneAnimationItem/OldMan_Spline/BP_Item.BP_Item_C|SetSplineToFollow _returnvalue (Variables|/Game/BluePrints/Item/SceneAnimationItem/OldMan_Spline/BP_Item.BP_Item_C|GetSplineToFollow _item))
      (Variables|/Game/BluePrints/Item/SceneAnimationItem/OldMan_Spline/BP_Item.BP_Item_C|SetItemMesh _returnvalue (Variables|/Game/BluePrints/Item/SceneAnimationItem/OldMan_Spline/BP_Item.BP_Item_C|GetItemMesh _item))
      (Variables|/Game/BluePrints/Item/SceneAnimationItem/OldMan_Spline/BP_Item.BP_Item_C|SetFloatRate _returnvalue (Variables|/Game/BluePrints/Item/SceneAnimationItem/OldMan_Spline/BP_Item.BP_Item_C|GetFloatRate _item))
      (Variables|/Game/BluePrints/Item/SceneAnimationItem/OldMan_Spline/BP_Item.BP_Item_C|SetFloatExtremum _returnvalue (Variables|/Game/BluePrints/Item/SceneAnimationItem/OldMan_Spline/BP_Item.BP_Item_C|GetFloatExtremum _item))
      (Variables|/Game/BluePrints/Item/SceneAnimationItem/OldMan_Spline/BP_Item.BP_Item_C|SetLoop _returnvalue (Variables|/Game/BluePrints/Item/SceneAnimationItem/OldMan_Spline/BP_Item.BP_Item_C|GetLoop _item))
      (Variables|/Game/BluePrints/Item/SceneAnimationItem/OldMan_Spline/BP_Item.BP_Item_C|SetReserveStart _returnvalue (Variables|/Game/BluePrints/Item/SceneAnimationItem/OldMan_Spline/BP_Item.BP_Item_C|GetReserveStart _item))
      (Variables|/Game/BluePrints/Item/SceneAnimationItem/OldMan_Spline/BP_Item.BP_Item_C|SetIsFloat _returnvalue (Variables|/Game/BluePrints/Item/SceneAnimationItem/OldMan_Spline/BP_Item.BP_Item_C|GetIsFloat _item))
      (Class|TimelineComponent|SetFloatCurve (Variables|/Game/BluePrints/Item/SceneAnimationItem/OldMan_Spline/BP_Item.BP_Item_C|GetMoveTimeLine _returnvalue) (Variables|/Game/BluePrints/Item/SceneAnimationItem/OldMan_Spline/BP_Item.BP_Item_C|GetFloatCurve _item) "None")
      (Variables|/Game/BluePrints/Item/SceneAnimationItem/OldMan_Spline/BP_Item.BP_Item_C|SetTime _returnvalue (Variables|/Game/BluePrints/Item/SceneAnimationItem/OldMan_Spline/BP_Item.BP_Item_C|GetTime _item))
      (Default|MoveItem _returnvalue))))

(fn ConstructionScript)