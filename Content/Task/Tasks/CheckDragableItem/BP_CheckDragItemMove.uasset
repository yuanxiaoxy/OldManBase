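; Task Blueprint for a tutorial step, named as a check that the player moves a draggable item.
; On start it opens the mouse-move guide popup additively and caches it as an old-man popup panel.
; On completion it tells that panel the player's action is finished, then spawns an animation trigger that plays a language-specific HAP alpha video on the UI with a transparent material.
; The completion check itself is not in this graph.
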(event EventOnStartTask
  (Development|PrintText "Hello")
  (bind _returnvalue (Class|UIManager|ShowUIbyName (Class|UIManager|GetUIManager) "PopupPanel_Guide_MouseMove" 0 "Additive"))
  (bind _asold_man_pop_up_uibase (Utilities|Casting|CastToOldManPopUpUIBase _returnvalue))
  (Variables|Default|SetCachePanel _asold_man_pop_up_uibase))

(event EventOnCompleteTask
  (Development|PrintText "Finish")
  (Class|OldManPopUpUIBase|FinishPlayerAction (Variables|Default|GetCachePanel))
  (bind _returnvalue (Game|SpawnActorfromClass "/Game/BluePrints/Item/AnimationBall/BP_AnimationBallTrigger.BP_AnimationBallTrigger_C" (Math|Conversions|ToTransform(Vector) "0, 0, 0") "Undefined" "MultiplyWithRoot" 0 false "None" 0))
  (Variables|/Script/OldManItem.OldManAnimationBall|SetFileMediaSourceInEnglish _returnvalue "/Game/Movies/AnimationBallMovies/L1/Real/English/Try_4_HAP_Alpha.Try_4_HAP_Alpha")
  (Variables|/Script/OldManItem.OldManAnimationBall|SetFileMediaSource _returnvalue "/Game/Movies/AnimationBallMovies/L1/Real/CaoZuo4_HAP_Alpha.CaoZuo4_HAP_Alpha")
  (Variables|/Script/OldManItem.OldManAnimationBall|SetPlayWallMaterial _returnvalue "/Game/Movies/AnimationBall/ABT_TouMing_Mat.ABT_TouMing_Mat")
  (Variables|/Script/OldManItem.OldManAnimationBall|SetmyType _returnvalue "playOnUI")
  (Variables|/Script/OldManItem.OldManAnimationBall|SetPlayerInputCancel _returnvalue false)
  (Class|OldManAnimationBall|PlayVideoinUI _returnvalue))