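; BP_BossGrid is a boss-fight grid actor that reports to the level manager whether the player is in danger or safe.
; On BeginPlay it finds the BP_BossLevelManager in the level and caches it as its receiver.
; Its OnPlayerinDanger and OnPlayerinSafe events check the passed actor for the player tag, then call the matching PlayerInDanger or PlayerInSafe on the manager.
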(event EventBeginPlay
  (bind _returnvalue (Actor|GetActorOfClass "/Game/Boss/BP_BossLevelManager.BP_BossLevelManager_C"))
  (Variables|Default|SetRecevier _returnvalue))

(event Collision|EventActorBeginOverlap
  (params (OtherActor :type Actor%20Object%20Reference)))

(event EventTick
  (params (DeltaSeconds :type Float%20%28single-precision%29)))

(event EventOnPlayerinDanger
  (params (OtherActor :type Actor%20Object%20Reference))
  (bind _returnvalue (Class|GlobalTagName|GetTagPlayer))
  (if (> (Utilities|Array|FindItem (Variables|/Script/Engine.Actor|GetTags OtherActor) _returnvalue) -1)
    (Default|PlayerinDanger (Variables|Default|GetRecevier))))

(event EventOnPlayerinSafe
  (params (OtherActor :type Actor%20Object%20Reference))
  (bind _returnvalue (Class|GlobalTagName|GetTagPlayer))
  (if (> (Utilities|Array|FindItem (Variables|/Script/Engine.Actor|GetTags OtherActor) _returnvalue) -1)
    (Default|PlayerinSafe (Variables|Default|GetRecevier))))

(fn ConstructionScript)