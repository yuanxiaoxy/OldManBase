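; BP_WaterArea is a water volume that tells the player's OldManCharacter when it is inside water.
; A trigger-enter event sets InWater on the character, and the AreaBox end-overlap event clears it.
; Both events act only on actors carrying the player tag that cast successfully to OldManCharacter.
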(event OnComponentEndOverlap(AreaBox)
  (params (OverlappedComponent :type Primitive%20Component%20Object%20Reference) (OtherActor :type Actor%20Object%20Reference) (OtherComp :type Primitive%20Component%20Object%20Reference) (OtherBodyIndex :type Integer))
  (bind _returnvalue (Class|GlobalTagName|GetTagPlayer))
  (if (> (Utilities|Array|FindItem (Variables|/Script/Engine.Actor|GetTags OtherActor) _returnvalue) -1)
    (bind _asold_man_character (Utilities|Casting|CastToOldManCharacter OtherActor))
    (Variables|/Script/OldMan.OldManCharacter|SetbInWater _asold_man_character false)))

(event EventOnEnterTrigger
  (params (OverlappedComponent :type Primitive%20Component%20Object%20Reference) (OtherActor :type Actor%20Object%20Reference) (OtherComp :type Primitive%20Component%20Object%20Reference) (OtherBodyIndex :type Integer) (bFromSweep :type Boolean) (SweepResult :type Hit%20Result%20Structure%20%28by%20ref%29))
  (bind _returnvalue (Class|GlobalTagName|GetTagPlayer))
  (if (> (Utilities|Array|FindItem (Variables|/Script/Engine.Actor|GetTags OtherActor) _returnvalue) -1)
    (bind _asold_man_character (Utilities|Casting|CastToOldManCharacter OtherActor))
    (Variables|/Script/OldMan.OldManCharacter|SetbInWater _asold_man_character true)))

(fn ConstructionScript)