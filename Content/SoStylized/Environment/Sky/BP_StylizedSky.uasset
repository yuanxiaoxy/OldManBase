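; Stylized sky actor that runs a looping day/night cycle with sun, moon, clouds, shooting stars with random meteor showers, and an optional planetary ring.
; Alternating day and night timelines rotate one shared directional light and the sun/moon meshes, publishing time and directions to MPC_GlobalEnvironment.
; Slower timers update skylight, volumetric fog and ring shadow, using a cyclic four-phase lerp for skylight and fog.
; The construction script applies orbit, materials and start time.
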(event Custom|Day%20Event
  ;[1 0.7481 0.2744] Day and Sun
  (bind (_direction _curvevalue _brightness _daycycleprogress) (Timeline|DayTimeline Play)
    (:Update
      (CallFunction|HandleDayTimeline _curvevalue _brightness _daycycleprogress))
    (:Finished
      (Components|Timeline|SetNewTime (Variables|Default|GetNightTimeline) 0.0)
      (CallFunction|NightEvent))))

(event Custom|Night%20Event
  ;[0.2327 0.4667 1] Night and moon
  (bind (_direction _curvevalue _brightness _daycycleprogress _shootingstarrate) (Timeline|NightTimeline Play)
    (:Update
      (CallFunction|HandleNightTimeline _curvevalue _brightness _daycycleprogress _shootingstarrate))
    (:Finished
      (Components|Timeline|SetNewTime (Variables|Default|GetDayTimeline) 0.0)
      (CallFunction|DayEvent))
    (:BeginShootingStars
      (CallFunction|BeginShootingStars))
    (:EndShootingStars
      (CallFunction|StopShootingStars))))

(event EventBeginPlay
  (Utilities|FlowControl|Sequence
    (:then_0
      ;[1 1 1] We update some of our MPC values when we begin the game just to be safe. Doesn't seem to work otherwise. We also update our timeline lengths now based on our day/night times.
      (Rendering|Material|SetScalarParameterValue "/Game/SoStylized/Environment/MPC_GlobalEnvironment.MPC_GlobalEnvironment" "Day Length" (Variables|01Day/NightCycle|GetDay%20Length) :!class /Script/Engine.KismetMaterialLibrary)
      (Rendering|Material|SetScalarParameterValue "/Game/SoStylized/Environment/MPC_GlobalEnvironment.MPC_GlobalEnvironment" "Night Length" (Variables|01Day/NightCycle|GetNight%20Length) :!class /Script/Engine.KismetMaterialLibrary)
      (Components|Timeline|SetPlayRate (Variables|Default|GetDayTimeline) (/ 1.0 (Variables|01Day/NightCycle|GetDay%20Length)))
      (Components|Timeline|SetPlayRate (Variables|Default|GetNightTimeline) (/ 1.0 (Variables|01Day/NightCycle|GetNight%20Length))))
    (:then_1
      (Rendering|Material|SetScalarParameterValue "/Game/SoStylized/Environment/MPC_GlobalEnvironment.MPC_GlobalEnvironment" "Orbit Orientation" (Variables|02Planetary|GetOrbit%20Orientation) :!class /Script/Engine.KismetMaterialLibrary)
      (Rendering|Material|SetScalarParameterValue "/Game/SoStylized/Environment/MPC_GlobalEnvironment.MPC_GlobalEnvironment" "Orbit Inclination" (Variables|02Planetary|GetOrbit%20Inclination) :!class /Script/Engine.KismetMaterialLibrary))
    (:then_2
      ;[1 1 1] Same as in construction script, update our current time of day, set time, and then begin the actual timeline event.
      (bind _output_get (Variables|Default|SetCurrent%20Time%20of%20Day (Math|Float|%(Float) (Variables|01Day/NightCycle|GetStart%20Time) (+ (Variables|01Day/NightCycle|GetDay%20Length) (Variables|01Day/NightCycle|GetNight%20Length)))))
      (if (> _output_get (Variables|01Day/NightCycle|GetDay%20Length)) ; If our start time is greater than\nour day length, then we're\nactually starting at night.
        (Components|Timeline|SetNewTime (Variables|Default|GetNightTimeline) (/ (- (Variables|01Day/NightCycle|GetStart%20Time) (Variables|01Day/NightCycle|GetDay%20Length)) (Variables|01Day/NightCycle|GetNight%20Length)))
        (CallFunction|NightEvent)
        (else
          (Components|Timeline|SetNewTime (Variables|Default|GetDayTimeline) (/ (Variables|01Day/NightCycle|GetStart%20Time) (Variables|01Day/NightCycle|GetDay%20Length)))
          (CallFunction|DayEvent))))
    (:then_3
      ;[1 1 1] The movement of the sun/moon across the sky we will be updating at a clean 60fps (the actor tick rate) but for some subtle things like skylight color we can update at a much lower frequency and it's really not noticeable. Good performance! By default it's only updating these things like every 5 seconds.
      ;
      ; To find a good interval rate, we take whatever is shorter, day or night, anddivy it up into fractions. Anything more isn't perceivable.
      (bind _output_get_2 (Variables|Default|SetSky%20Update%20Interval (Math|Float|Max(Float) (/ (Math|Float|Min(Float) (Variables|01Day/NightCycle|GetDay%20Length) (Variables|01Day/NightCycle|GetNight%20Length)) 9e+01) 0.016667)))
      (Utilities|Time|SetTimerbyFunctionName 0 "Update Lights" _output_get_2 true))
    (:then_4
      ;[1 1 1] Setting the ring shadow update function, assuming we have a ring and ring shadow.
      (if (and (Variables|02Planetary|GetPlanetaryRing?) (> (Variables|02Planetary|GetRing%20Shadow%20Strength) 0.0)) ; We don't need to update the shadow on the\nring if we don't have a ring. Also if we have\nour shadow amount set to 0, we also have\nno need to update this.
        (Utilities|Time|SetTimerbyFunctionName 0 "Update Ring Shadow" 0.033333 true)))))

(fn ConstructionScript
  (bind _planetaryring_ (Variables|02Planetary|GetPlanetaryRing?))
  (Utilities|FlowControl|Sequence
    (:then_0
      ;[1 1 1] Set the material parameter collection (MPC) values for our day and night lengths based on what we set on our BP. Also update the play rate of the day/night timelines accordingly.
      (Rendering|Material|SetScalarParameterValue "/Game/SoStylized/Environment/MPC_GlobalEnvironment.MPC_GlobalEnvironment" "Day Length" (Variables|01Day/NightCycle|GetDay%20Length) :!class /Script/Engine.KismetMaterialLibrary)
      (Rendering|Material|SetScalarParameterValue "/Game/SoStylized/Environment/MPC_GlobalEnvironment.MPC_GlobalEnvironment" "Night Length" (Variables|01Day/NightCycle|GetNight%20Length) :!class /Script/Engine.KismetMaterialLibrary))
    (:then_1
      ;[1 1 1] Rotate the orbit and inclination of our sun/moon trajectories (and then update the MPC as well.)
      (Transformation|SetRelativeRotation (Variables|Default|GetOrbitOrientator) (Math|Rotator|MakeRotator 0.0 0.0 (+ (Variables|02Planetary|GetOrbit%20Orientation) 9e+01)) false false)
      (Transformation|SetRelativeRotation (Variables|Default|GetOrbitInclinator) (Math|Rotator|MakeRotator (Variables|02Planetary|GetOrbit%20Inclination) 0.0 0.0) false false)
      (Transformation|SetRelativeRotation (Variables|Default|GetSkyDome) (Math|Rotator|MakeRotator 0.0 0.0 (+ (Variables|02Planetary|GetOrbit%20Orientation) 9e+01)) false false)
      (Rendering|Material|SetScalarParameterValue "/Game/SoStylized/Environment/MPC_GlobalEnvironment.MPC_GlobalEnvironment" "Orbit Orientation" (Variables|02Planetary|GetOrbit%20Orientation) :!class /Script/Engine.KismetMaterialLibrary)
      (Rendering|Material|SetScalarParameterValue "/Game/SoStylized/Environment/MPC_GlobalEnvironment.MPC_GlobalEnvironment" "Orbit Inclination" (Variables|02Planetary|GetOrbit%20Inclination) :!class /Script/Engine.KismetMaterialLibrary))
    (:then_2
      ;[1 1 1] Update our start time (with looping) and then set our new current time in the appropriate timeline. This will also update the timeline output once and update our sky and materials.
      (bind _output_get (Variables|01Day/NightCycle|SetStart%20Time (Math|Float|%(Float) (Variables|01Day/NightCycle|GetStart%20Time) (+ (Variables|01Day/NightCycle|GetDay%20Length) (Variables|01Day/NightCycle|GetNight%20Length)))))
      (if (> _output_get (Variables|01Day/NightCycle|GetDay%20Length)) ; If our start time is greater than\nour day length, then we're\nactually starting at night.
        (Components|Timeline|SetNewTime (Variables|Default|GetNightTimeline) (/ (- (Variables|01Day/NightCycle|GetStart%20Time) (Variables|01Day/NightCycle|GetDay%20Length)) (Variables|01Day/NightCycle|GetNight%20Length)))
        (CallFunction|NightEvent)
        (else
          (Components|Timeline|SetNewTime (Variables|Default|GetDayTimeline) (/ (Variables|01Day/NightCycle|GetStart%20Time) (Variables|01Day/NightCycle|GetDay%20Length)))
          (CallFunction|DayEvent))))
    (:then_3
      ;[1 1 1] Update some of our materials for post process, sun, moon, volumetric fog, and lights.
      (Utilities|Struct|SetmembersinPostProcessSettings (Variables|/Script/Engine.PostProcessComponent|GetSettings (Variables|Default|GetPostProcess)) (Utilities|Struct|MakeWeightedBlendables (Utilities|Array|MakeArray (Utilities|Struct|MakeWeightedBlendable 1.0 (Variables|04Fog|GetPost%20Process%20Fog%20Material)))))
      (Rendering|SetVisibility (Variables|Default|GetExponentialHeightFog) (Variables|04Fog|GetVolumetricFog?) false)
      (Rendering|Material|SetMaterial (Variables|Default|GetSM_Sun) 0 (Variables|03Sun,Moon,Light|GetSun%20Material))
      (Rendering|Material|SetMaterial (Variables|Default|GetSM_Moon) 0 (Variables|03Sun,Moon,Light|GetMoon%20Material))
      (Rendering|Components|Light|SetLightFunctionMaterial (Variables|Default|GetSkyDirectionalLight) (select (Variables|05Sky&Clouds|GetCloud%20Shadows?) "/Game/SoStylized/Environment/Sky/Materials/MI_SunCloudShadows_LF.MI_SunCloudShadows_LF" 0))
      (CallFunction|UpdateLights))
    (:then_4
      ;[1 1 1] All about the optional planetary ring. Setting up its location, rotation, materials, etc.
      (Rendering|SetVisibility (Variables|Default|GetRing) _planetaryring_ false)
      (if _planetaryring_
        (Transformation|SetRelativeRotation (Variables|Default|GetRing) (Math|Rotator|MakeRotator (+ 2.7e+02 (Variables|02Planetary|GetRing%20Pitch)) 0.0 (+ (- (Variables|02Planetary|GetOrbit%20Orientation) 1.1e+02) (Variables|02Planetary|GetRing%20Orientation))) false false)
        (Transformation|SetRelativeLocation (Variables|Default|GetRing) (Math|Vector|MakeVector 0.0 0.0 (* (- (Variables|02Planetary|GetRing%20Vertical%20Offset) 7.0) 1e+06)) false false)
        (bind _returnvalue (Rendering|Material|CreateDynamicMaterialInstance (Variables|Default|GetRing) 0 "/Game/SoStylized/Environment/Sky/Materials/MI_PlanetRing_Inst.MI_PlanetRing_Inst" "None" :!class /Script/Engine.PrimitiveComponent))
        (Variables|02Planetary|SetDMI_PlanetRing _returnvalue)
        (CallFunction|UpdateRingShadow)
        (Rendering|Material|SetScalarParameterValue (Variables|02Planetary|GetDMI_PlanetRing) "Strength" (Variables|02Planetary|GetRing%20Strength) :!class /Script/Engine.MaterialInstanceDynamic)
        (Rendering|Material|SetScalarParameterValue (Variables|02Planetary|GetDMI_PlanetRing) "Planet Shadow Strength" (Variables|02Planetary|GetRing%20Shadow%20Strength) :!class /Script/Engine.MaterialInstanceDynamic)
        (Rendering|Material|SetVectorParameterValue (Variables|02Planetary|GetDMI_PlanetRing) "Color 1" (Variables|02Planetary|GetRing%20Color%201) :!class /Script/Engine.MaterialInstanceDynamic)
        (Rendering|Material|SetVectorParameterValue (Variables|02Planetary|GetDMI_PlanetRing) "Color 2" (Variables|02Planetary|GetRing%20Color%202) :!class /Script/Engine.MaterialInstanceDynamic)))
    (:then_5
      ;[1 1 1] The sky dome and sky cloud dome.
      (Rendering|Material|SetMaterial (Variables|Default|GetSkyDome) 0 (Variables|05Sky&Clouds|GetSky%20Material))
      (Rendering|SetVisibility (Variables|Default|GetSkyDomeClouds) (Variables|05Sky&Clouds|GetClouds?) false)
      (if (Variables|05Sky&Clouds|GetClouds?)
        (Rendering|Material|SetMaterial (Variables|Default|GetSkyDomeClouds) 0 (Variables|05Sky&Clouds|GetCloud%20Material))))
    (:then_6
      ;[1 1 1] Shooting stars
      (Transformation|SetRelativeRotation (Variables|Default|GetShooting%20Stars) (Math|Rotator|MakeRotator 0.0 0.0 (Variables|06ShootingStars|GetShooting%20Star%20Orientation)) false false))))

(fn UpdateLightRotation
  (bind _sm_sun (Variables|Default|GetSM_Sun))
  (bind _sm_moon (Variables|Default|GetSM_Moon))
  (bind _returnvalue (Transformation|GetWorldRotation _sm_sun))
  (bind _returnvalue_2 (Transformation|GetWorldRotation _sm_moon))
  (bind (_roll _pitch _yaw) (Math|Rotator|BreakRotator _returnvalue))
  (bind (_roll_2 _pitch_2 _yaw_2) (Math|Rotator|BreakRotator _returnvalue_2))
  (Utilities|FlowControl|Sequence
    (:then_0
      ;[1 1 1] First we update our Sky Light's "Rotation" using Rotators. This makes it much easier to Lerp a lot of
      ; the time of day settings, as rotators have clean pitch and yaw values.
      (Rendering|Material|SetVectorParameterValue "/Game/SoStylized/Environment/MPC_GlobalEnvironment.MPC_GlobalEnvironment" "Sun Light Rotation" (Math|Color|MakeColor _roll _pitch _yaw) :!class /Script/Engine.KismetMaterialLibrary)
      ;[1 1 1] We also update the "direction" the sky light is facing, which is more useful for dot products to tell when the light passes behind clouds to illuminate them and similar.
      (Rendering|Material|SetVectorParameterValue "/Game/SoStylized/Environment/MPC_GlobalEnvironment.MPC_GlobalEnvironment" "Sun Light Direction" (Math|Conversions|ToLinearColor(Vector) (Math|Vector|GetForwardVector (Variables|Default|GetSM_Sun))) :!class /Script/Engine.KismetMaterialLibrary))
    (:then_1
      ;[1 1 1] Same process for the moon's rotation.
      (Rendering|Material|SetVectorParameterValue "/Game/SoStylized/Environment/MPC_GlobalEnvironment.MPC_GlobalEnvironment" "Moon Light Rotation" (Math|Color|MakeColor _roll_2 _pitch_2 _yaw_2) :!class /Script/Engine.KismetMaterialLibrary)
      ;[1 1 1] And the moon direction.
      (Rendering|Material|SetVectorParameterValue "/Game/SoStylized/Environment/MPC_GlobalEnvironment.MPC_GlobalEnvironment" "Moon Light Direction" (Math|Conversions|ToLinearColor(Vector) (Math|Vector|GetForwardVector (Variables|Default|GetSM_Moon))) :!class /Script/Engine.KismetMaterialLibrary))))

(fn UpdateLights
  (bind _exponentialheightfog (Variables|Default|GetExponentialHeightFog))
  (Rendering|Components|Light|SetIntensity (Variables|Default|GetSkyLight) (CallFunction|DayCycleLerpFloat (Variables|03Sun,Moon,Light|GetDay%20Skylight%20Intensity) (Variables|03Sun,Moon,Light|GetSunset%20Skylight%20Intensity) (Variables|03Sun,Moon,Light|GetNight%20%20Skylight%20Intensity) (Variables|03Sun,Moon,Light|GetSunrise%20Skylight%20Intensity)))
  (Rendering|Components|Light|SetLightColor (Variables|Default|GetSkyLight) (CallFunction|DayCycleLerpColor (Variables|03Sun,Moon,Light|GetDay%20Skylight%20Color) (Variables|03Sun,Moon,Light|GetSunset%20Skylight%20Color) (Variables|03Sun,Moon,Light|GetNight%20Skylight%20Color) (Variables|03Sun,Moon,Light|GetSunrise%20Skylight%20Color)))
  (if (Variables|04Fog|GetVolumetricFog?)
    (Class|ExponentialHeightFogComponent|SetFogDensity _exponentialheightfog (CallFunction|DayCycleLerpFloat (Variables|04Fog|GetDay%20Volumetric%20Density) (Variables|04Fog|GetSunset%20Volumetric%20Density) (Variables|04Fog|GetNight%20Volumetric%20Density) (Variables|04Fog|GetSunrise%20Volumetric%20Density)))
    (Class|ExponentialHeightFogComponent|SetVolumetricFogAlbedo _exponentialheightfog (Math|Conversions|ToColor(LinearColor) (CallFunction|DayCycleLerpColor (Variables|04Fog|GetDay%20Volumetric%20Fog%20Color) (Variables|04Fog|GetSunset%20Volumetric%20Fog%20Color) (Variables|04Fog|GetNight%20Volumetric%20Fog%20Color) (Variables|04Fog|GetSunrise%20Volumetric%20Fog%20Color))))))

(fn UpdateRingShadow
  (bind _dmi_planetring (Variables|02Planetary|GetDMI_PlanetRing))
  (Utilities|IsValid _dmi_planetring
    (:Is%20Valid
      (Rendering|Material|SetScalarParameterValue _dmi_planetring "Rotation" (/ (Variables|Default|GetCurrent%20Time%20of%20Day) (+ (Variables|01Day/NightCycle|GetDay%20Length) (Variables|01Day/NightCycle|GetNight%20Length))) :!class /Script/Engine.MaterialInstanceDynamic))))

(fn HandleDayTimeline
  (params (Curve%20Alpha :type Float%20%28double-precision%29) (Day%20Brightness :type Float%20%28single-precision%29) (New%20Progress :type Float%20%28single-precision%29))
  (Utilities|FlowControl|Sequence
    (:then_0
      (Transformation|SetRelativeRotation (Variables|Default|GetSkyDirectionalLight) (Math|Rotator|MakeRotator (Math|Float|Lerp (Variables|02Planetary|GetOrbit%20Inclination) (* (Variables|02Planetary|GetOrbit%20Inclination) -1.0) Curve%20Alpha) (Math|Float|Lerp 1.7e+02 3.7e+02 Curve%20Alpha) 0.0) false false)
      (Transformation|SetRelativeRotation (Variables|Default|GetSM_Moon) (Math|Rotator|MakeRotator 0.0 (Math|Float|Lerp 3.7e+02 5.3e+02 Curve%20Alpha) 0.0) false false)
      (CallFunction|UpdateLightRotation))
    (:then_1
      (Rendering|Components|Light|SetIntensity (Variables|Default|GetSkyDirectionalLight) (* Day%20Brightness (Variables|03Sun,Moon,Light|GetSunBrightness))))
    (:then_2
      (bind _output_get (Variables|Default|SetCurrent%20Time%20of%20Day (* Curve%20Alpha (Variables|01Day/NightCycle|GetDay%20Length))))
      (Rendering|Material|SetScalarParameterValue "/Game/SoStylized/Environment/MPC_GlobalEnvironment.MPC_GlobalEnvironment" "Current Time" _output_get :!class /Script/Engine.KismetMaterialLibrary)
      (Rendering|Components|Light|SetLightColor (Variables|Default|GetSkyDirectionalLight) (Math|Curves|GetLinearColorValue (Variables|03Sun,Moon,Light|GetSunColorCurve) (/ (Variables|Default|GetCurrent%20Time%20of%20Day) (Variables|01Day/NightCycle|GetDay%20Length))) true))
    (:then_3
      (bind _output_get_2 (Variables|Default|SetDay%20Cycle%20Progress New%20Progress))
      (Rendering|Material|SetScalarParameterValue "/Game/SoStylized/Environment/MPC_GlobalEnvironment.MPC_GlobalEnvironment" "Day Cycle Progress" _output_get_2 :!class /Script/Engine.KismetMaterialLibrary))))

(fn HandleNightTimeline
  (params (Curve%20Alpha :type Float%20%28double-precision%29) (Night%20Brightness :type Float%20%28single-precision%29) (New%20Progress :type Float%20%28single-precision%29) (Shooting%20Star%20Rate :type Float%20%28double-precision%29))
  (Utilities|FlowControl|Sequence
    (:then_0
      (Transformation|SetRelativeRotation (Variables|Default|GetSkyDirectionalLight) (Math|Rotator|MakeRotator (Math|Float|Lerp (Variables|02Planetary|GetOrbit%20Inclination) (* (Variables|02Planetary|GetOrbit%20Inclination) -1.0) Curve%20Alpha) (Math|Float|Lerp 1.7e+02 3.7e+02 Curve%20Alpha) 0.0) false false)
      (Transformation|SetRelativeRotation (Variables|Default|GetSM_Sun) (Math|Rotator|MakeRotator (Variables|02Planetary|GetOrbit%20Inclination) (Math|Float|Lerp 3.7e+02 5.3e+02 Curve%20Alpha) 0.0) false false)
      (CallFunction|UpdateLightRotation))
    (:then_1
      (Rendering|Components|Light|SetIntensity (Variables|Default|GetSkyDirectionalLight) (* Night%20Brightness (Variables|03Sun,Moon,Light|GetMoonBrightness))))
    (:then_2
      (bind _output_get (Variables|Default|SetCurrent%20Time%20of%20Day (+ (Variables|01Day/NightCycle|GetDay%20Length) (* Curve%20Alpha (Variables|01Day/NightCycle|GetNight%20Length)))))
      (Rendering|Material|SetScalarParameterValue "/Game/SoStylized/Environment/MPC_GlobalEnvironment.MPC_GlobalEnvironment" "Current Time" _output_get :!class /Script/Engine.KismetMaterialLibrary)
      (Rendering|Components|Light|SetLightColor (Variables|Default|GetSkyDirectionalLight) (Math|Curves|GetLinearColorValue (Variables|03Sun,Moon,Light|GetMoonColorCurve) (/ (- (Variables|Default|GetCurrent%20Time%20of%20Day) (Variables|01Day/NightCycle|GetDay%20Length)) (Variables|01Day/NightCycle|GetNight%20Length))) true))
    (:then_3
      (bind _output_get_2 (Variables|Default|SetDay%20Cycle%20Progress New%20Progress))
      (Rendering|Material|SetScalarParameterValue "/Game/SoStylized/Environment/MPC_GlobalEnvironment.MPC_GlobalEnvironment" "Day Cycle Progress" _output_get_2 :!class /Script/Engine.KismetMaterialLibrary))
    (:then_4
      (Niagara|SetNiagaraVariable(Float) (Variables|Default|GetShooting%20Stars) "SpawnRate" (* Shooting%20Star%20Rate (select (Variables|06ShootingStars|GetMeteorShowerNight?) (Variables|06ShootingStars|GetShooting%20Star%20Frequency%20During%20Meteor%20Shower) (Variables|06ShootingStars|GetShooting%20Star%20Frequency)))))))

(fn BeginShootingStars
  (Components|Activation|Activate (Variables|Default|GetShooting%20Stars) true)
  (Variables|06ShootingStars|SetMeteorShowerNight? (< (* (Math|Random|RandomFloat) 1e+02) (Variables|06ShootingStars|GetMeteor%20Shower%20Chance))))

(fn StopShootingStars
  (Components|Activation|Deactivate (Variables|Default|GetShooting%20Stars)))

(fn DayCycleLerpFloat
  (params (Day :type Float%20%28double-precision%29) (Sunset :type Float%20%28double-precision%29) (Night :type Float%20%28double-precision%29) (Sunrise :type Float%20%28double-precision%29))
  (bind _day_cycle_progress (Variables|Default|GetDay%20Cycle%20Progress))
  (bind _returnvalue (* _day_cycle_progress 4.0))
  (bind _returnvalue_2 (- _returnvalue 1.0))
  (bind _returnvalue_3 (- _returnvalue_2 1.0))
  ;[1 1 1] This is essentially the same 5-way lerp I have as a material function. It's a cheap and easy way to blend between five values (or more specifically, blend between 4 values where the last value is the same as the first, that way it creates a cycling loop.)
  (return (Math|Float|Lerp (Math|Float|Lerp (Math|Float|Lerp (Math|Float|Lerp Day Sunset (Math|Float|Clamp(Float) _returnvalue)) Night (Math|Float|Clamp(Float) _returnvalue_2)) Sunrise (Math|Float|Clamp(Float) _returnvalue_3)) Day (Math|Float|Clamp(Float) (- _returnvalue_3 1.0)))))

(fn DayCycleLerpColor
  (params (Day :type Linear%20Color%20Structure) (Sunset :type Linear%20Color%20Structure) (Night :type Linear%20Color%20Structure) (Sunrise :type Linear%20Color%20Structure))
  (bind _day_cycle_progress (Variables|Default|GetDay%20Cycle%20Progress))
  (bind _returnvalue (* _day_cycle_progress 4.0))
  (bind _returnvalue_2 (- _returnvalue 1.0))
  (bind _returnvalue_3 (- _returnvalue_2 1.0))
  ;[1 1 1] This is essentially the same 5-way lerp I have as a material function. It's a cheap and easy way to blend between five values (or more specifically, blend between 4 values where the last value is the same as the first, that way it creates a cycling loop.)
  (return (Math|Color|Lerp(LinearColor) (Math|Color|Lerp(LinearColor) (Math|Color|Lerp(LinearColor) (Math|Color|Lerp(LinearColor) Day Sunset (Math|Float|Clamp(Float) _returnvalue)) Night (Math|Float|Clamp(Float) _returnvalue_2)) Sunrise (Math|Float|Clamp(Float) _returnvalue_3)) Day (Math|Float|Clamp(Float) (- _returnvalue_3 1.0)))))