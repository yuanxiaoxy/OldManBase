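; BP_CheckPlayerInJump is a task that shows a pop-up UI for the player jump step and completes after a fixed delay.
; On start it opens the UI by name, caches it as an OldManPopUpUIBase and sets a MonoManager timer that completes the task.
; On completion it calls FinishPlayerAction on the cached panel.
; Despite the name, it never reads the player's jump state, and its tick is empty.
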(event Custom|OnFinished
  (Class|TaskBase|CompleteTask))

(event EventOnStartTask
  (bind _returnvalue (Class|UIManager|ShowUIbyName (Class|UIManager|GetUIManager) (Variables|Default|GetUIName) 0 "Additive" -1))
  (bind _asold_man_pop_up_uibase (Utilities|Casting|CastToOldManPopUpUIBase _returnvalue))
  (Variables|Default|SetCachePanel _asold_man_pop_up_uibase)
  (Class|MonoManager|SetTimeoutSimplewithId (Class|MonoManager|GetMonoManager) 2.5 "PopupUI_Jump" (delegate Custom|OnFinished)))

(event EventOnTick
  (params (DeltaTime :type Float%20%28single-precision%29)))

(event EventOnCompleteTask
  (bind _cachepanel (Variables|Default|GetCachePanel))
  (Utilities|IsValid _cachepanel
    (:Is%20Valid
      (Class|OldManPopUpUIBase|FinishPlayerAction _cachepanel))))