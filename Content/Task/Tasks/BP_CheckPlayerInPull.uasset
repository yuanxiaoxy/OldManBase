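; Tutorial task that waits for the player to enter the pull state.
; On start it fires the event that unlocks pull key input, spawns an animation ball trigger to play an alpha guide video on the UI, and additively shows the mouse-move guide popup.
; Each tick it polls the cached player's InPullState, completes once that is true, then tells the cached popup the player action is finished.
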(event EventOnStartTask
  (bind _returnvalue (Class|GlobalEventName|GetKeyInputUnLockPull))
  (Class|MyEventManager|TriggerCppEventUniversal (Class|MyEventManager|GetEventManager) _returnvalue (Utilities|Struct|MakeGameEventData))
  (bind _returnvalue_2 (Game|SpawnActorfromClass "/Game/BluePrints/Item/AnimationBall/BP_AnimationBallTrigger.BP_AnimationBallTrigger_C" (Math|Conversions|ToTransform(Vector) "0, 0, 0") "Undefined" "MultiplyWithRoot" 0 false "None" 0))
  (Variables|/Script/OldManItem.OldManAnimationBall|SetFileMediaSource _returnvalue_2 "/Game/Movies/AnimationBallMovies/L1/Real/CaoZuo3_HAP_Alpha_1.CaoZuo3_HAP_Alpha_1")
  (Variables|/Script/OldManItem.OldManAnimationBall|SetPlayWallMaterial _returnvalue_2 "/Game/Movies/AnimationBall/ABT_TouMing_Mat.ABT_TouMing_Mat")
  (Variables|/Script/OldManItem.OldManAnimationBall|SetmyType _returnvalue_2 "playOnUI")
  (Variables|/Script/OldManItem.OldManAnimationBall|SetPlayerInputCancel _returnvalue_2 false)
  (Class|OldManAnimationBall|PlayVideoinUI _returnvalue_2)
  (bind _returnvalue_3 (Class|UIManager|ShowUIbyName (Class|UIManager|GetUIManager) "PopupPanel_Guide_MouseMove" 0 "Additive"))
  (bind _asold_man_pop_up_uibase (Utilities|Casting|CastToOldManPopUpUIBase _returnvalue_3))
  (Variables|Default|SetCachePanel _asold_man_pop_up_uibase))

(event EventOnTick
  (params (DeltaTime :type Float%20%28single-precision%29))
  (bind _returnvalue (Class|TaskCheckPlayerAction|GetCachedPlayer))
  (Utilities|IsValid _returnvalue
    (:Is%20Valid
      (if (Variables|/Script/OldMan.OldManCharacter|GetbInPullState _returnvalue)
        (Class|TaskBase|CompleteTask)
        (else
          (Development|PrintText "Wait"))))))

(event EventOnCompleteTask
  (Development|PrintText "Hello")
  (Class|OldManPopUpUIBase|FinishPlayerAction (Variables|Default|GetCachePanel)))