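; Trigger actor for an animation ball, with effects on player contact and a video wall that fades in.
; Player-tagged overlap with InteractionBox plays a sound and, if BoomNIagara is set, an effect, both by ID through manager lookups.
; StartFadein, not called within this graph, runs a timeline driving the PlayWall material's OpacityMul.
; VideoPlayCompelete relays video completion through AnimationBallPlayCompelete.
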(event OnComponentBeginOverlap(InteractionBox)
  (params (OverlappedComponent :type Primitive%20Component%20Object%20Reference) (OtherActor :type Actor%20Object%20Reference) (OtherComp :type Primitive%20Component%20Object%20Reference) (OtherBodyIndex :type Integer) (bFromSweep :type Boolean) (SweepResult :type Hit%20Result%20Structure%20%28by%20ref%29))
  (bind _interactionbox (Variables|Default|GetInteractionBox))
  (bind _returnvalue (Class|GlobalTagName|GetTagPlayer))
  (if (> (Utilities|Array|FindItem (Variables|/Script/Engine.Actor|GetTags OtherActor) _returnvalue) -1)
    (Utilities|FlowControl|Sequence
      (:then_0
        (if (Variables|Default|GetBoomNIagara)
          (Class|EffectManager|PlayEffectatLocation (Class|EffectManager|GetEffectManager) (Variables|Default|GetEffectID) (Transformation|GetWorldLocation _interactionbox) (Variables|/Script/Engine.SceneComponent|GetRelativeRotation _interactionbox))))
      (:then_1
        (Class|AudioManager|PlaySound (Class|AudioManager|GetAudioManager) (Variables|Default|GetAudioID) 0 "0, 0, 0" 0.0 0.0 1.0)))))

(event EventBeginPlay)

(event Collision|EventActorBeginOverlap
  (params (OtherActor :type Actor%20Object%20Reference)))

(event EventVideoPlayCompelete
  (Default|CallAnimationBallPlayCompelete))

(event EventStartFadein
  (bind _opacity (Timeline|FadeIn Play)
    (:Update
      (Rendering|Material|SetScalarParameterValueonMaterials (Variables|/Script/Engine.StaticMeshActor|GetStaticMeshComponent (Variables|Default|GetPlayWall)) "OpacityMul" _opacity))))

(fn ConstructionScript)