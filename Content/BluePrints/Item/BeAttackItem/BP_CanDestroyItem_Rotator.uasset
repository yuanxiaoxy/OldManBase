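; A destructible item actor that rotates its mesh once when struck by an object carrying the detection tag.
; The mesh's hit event latches on the first contact of any kind, then checks the other actor's tags.
; On a match it caches the mesh's relative rotation and a timeline lerps it to a configured target rotation.
; An untagged first hit also sets the latch, blocking any later rotation.
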(event OnComponentHit(MeshComponent)
  (params (HitComponent :type Primitive%20Component%20Object%20Reference) (OtherActor :type Actor%20Object%20Reference) (OtherComp :type Primitive%20Component%20Object%20Reference) (NormalImpulse :type Vector :default "0, 0, 0") (Hit :type Hit%20Result%20Structure%20%28by%20ref%29))
  (if (not (Variables|Default|GetHasAttacked))
    (Variables|Default|SetHasAttacked true)
    (Development|PrintString "hitted")
    (if (> (Utilities|Array|FindItem (Variables|/Script/Engine.Actor|GetTags OtherActor) "tag_DetcedItem") -1)
      (Variables|Default|SetCacheRotation (Variables|/Script/Engine.SceneComponent|GetRelativeRotation (Variables|Default|GetMeshComponent)))
      (bind _新建轨道_0 (Timeline|Lerp Play)
        (:Update
          (Transformation|SetRelativeRotation (Variables|Default|GetMeshComponent) (Math|Rotator|Lerp(Rotator) (Variables|Default|GetCacheRotation) (Variables|Default|GetRotation) _新建轨道_0) false false))))))

(event EventBeginPlay)

(event Collision|EventActorBeginOverlap
  (params (OtherActor :type Actor%20Object%20Reference)))

(fn ConstructionScript)