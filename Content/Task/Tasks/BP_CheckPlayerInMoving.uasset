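; Task Blueprint in the game's task system, named for checking whether the player is moving, apparently an unfinished step.
; On start it plays the L1_CaoZuo1 voice line through the audio manager, attached to the player character.
; Its tick compares the cached player's move state to Walk but takes no action on the result.
; Completion only prints a placeholder message, and failure does nothing.
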(event EventOnFailTask)

(event EventOnStartTask
  (bind _returnvalue (Game|GetPlayerCharacter 0))
  (Class|AudioManager|PlayVoice (Class|AudioManager|GetAudioManager) _returnvalue "L1_CaoZuo1" _returnvalue -1.0 -1.0 1.0))

(event EventOnTick
  (params (DeltaTime :type Float%20%28single-precision%29))
  (bind _returnvalue (Class|TaskCheckPlayerAction|GetCachedPlayer))
  (Utilities|IsValid _returnvalue
    (:Is%20Valid
      (if (Utilities|Enum|Equal(Enum) (Variables|/Script/OldMan.OldManCharacter|GetCurPlayerMoveState _returnvalue) "Walk")
        _))))

(event EventOnCompleteTask
  (Development|PrintText "Hello"))