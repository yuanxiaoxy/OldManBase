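; BP_AniBallTriggerTrans is an animation-ball trigger variant that teleports the player once a video finishes playing.
; On overlap it runs the parent logic, then caches the other actor as Player if it carries the player tag.
; The VideoPlayCompelete event moves that cached actor, if still valid, to TargetPos and TargetRot.
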(event EventBeginPlay
  (|CallParentFunction) ; 此节点被禁用，将不会被调用。\n从引脚连出引线来编译功能。
)

(event Collision|EventActorBeginOverlap
  (params (OtherActor :type Actor%20Object%20Reference))
  (|CallParentFunction OtherActor)
  (bind _returnvalue (Class|GlobalTagName|GetTagPlayer))
  (if (> (Utilities|Array|FindItem (Variables|/Script/Engine.Actor|GetTags OtherActor) _returnvalue) -1)
    (Variables|Default|SetPlayer OtherActor)))

(event EventTick
  (params (DeltaSeconds :type Float%20%28single-precision%29)))

(event EventVideoPlayCompelete
  (if (Utilities|IsValid (Variables|Default|GetPlayer))
    (Transformation|SetActorLocationAndRotation (Variables|Default|GetPlayer) (Variables|Default|GetTargetPos) (Variables|Default|GetTargetRot))))

(fn ConstructionScript
  (|CallParentFunction))