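; Boss level manager that runs a three-phase fight where parts of a boss head must be moved on voice prompts.
; Phases cover eyes and chin, head turns, then both combined.
; Sound-finished bindings chain prompts and countdowns, while interval timers delay scan checks and poll head state, repeating failed steps.
; It drives BossHead, TipLight and ScanLight; floors, zipline, enemies and ambient-light cues are PrintString placeholders, and audio uses test IDs.
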(event Custom|P1_LeftEyebrow_AudioCompelete
  (params (SoundID :type Name))
  ;[1 1 1] 阶段1_1_张开左眼
  (EventDispatchers|UnbindEventfromOnSoundFinished (Class|AudioManager|GetAudioManager) (delegate Custom|P1_LeftEyebrow_AudioCompelete))
  (Class|OldManBossHead|SetPartActive (Variables|TargetActor|GetBossHead) "LeftEyebrow" true)
  (Class|OldManBossHead|LeftEyebrowBlink (Variables|TargetActor|GetBossHead))
  (Class|OldManTipLight|SwitchCanMoveMat (Variables|TargetActor|GetTipLight) true)
  (EventDispatchers|BindEventtoOnSoundFinished (Class|AudioManager|GetAudioManager) (delegate Custom|P1_LeftEyebrow_CountDownCompelete))
  ;;[1 1 1] 阶段1地板随机生成
  (Development|PrintString "阶段1地板随机生成")
  ;;[1 1 1] 倒计时音频
  (Class|AudioManager|PlaySound (Class|AudioManager|GetAudioManager) "Test5" 0 "0, 0, 0" 0.0 0.0 1.0)
  (Development|PrintString "倒计时音频"))

(event Custom|BossFightStart
  ;[1 1 1] 老人头升起
  (Development|PrintString "老人头升起")
  ;[1 1 1] 阶段1_1_张开左眼
  (Class|OldManTipLight|SwitchCanMoveMat (Variables|TargetActor|GetTipLight) false)
  (EventDispatchers|BindEventtoOnSoundFinished (Class|AudioManager|GetAudioManager) (delegate Custom|P1_LeftEyebrow_AudioCompelete))
  ;;[1 1 1] 播放请张开左眼音频
  (Class|AudioManager|PlaySound (Class|AudioManager|GetAudioManager) "TestYveYin" 0 "0, 0, 0" 0.0 0.0 1.0)
  (Development|PrintString "播放请张开左眼音频")
  (Class|OldManTipLight|SwitchOperationMat (Variables|TargetActor|GetTipLight) "LeftEyebrow"))

(event Custom|P3_Eyebrow
  (params (SoundID :type Name))
  ;[1 1 1] 阶段3_1_张开双眼，并左右转头
  (EventDispatchers|UnbindEventfromOnSoundFinished (Class|AudioManager|GetAudioManager) (delegate Custom|P3_Eyebrow))
  (Class|OldManBossHead|SetPartActive (Variables|TargetActor|GetBossHead) "Eyebrow" true)
  (Class|OldManTipLight|SwitchOperationMat (Variables|TargetActor|GetTipLight) "Eyebrow")
  (Class|OldManBossHead|LeftEarBlink (Variables|TargetActor|GetBossHead))
  (Class|OldManBossHead|RightEarBlink (Variables|TargetActor|GetBossHead))
  (Class|OldManTipLight|SwitchCanMoveMat (Variables|TargetActor|GetTipLight) true)
  (Class|OldManMobileCamera|BeginScanWithoutParm (Variables|TargetActor|GetScanLight))
  (EventDispatchers|BindEventtoOnSoundFinished (Class|AudioManager|GetAudioManager) (delegate Custom|P3_CountTimeCompelete))
  ;;[1 1 1] 倒计时
  (Class|AudioManager|PlaySound (Class|AudioManager|GetAudioManager) "Test30" 0 "0, 0, 0" 0.0 0.0 1.0)
  (Development|PrintString "倒计时")
  (Class|MonoManager|SetIntervalwithId (Class|MonoManager|GetMonoManager) 0.5 "CheckMoving" (delegate Custom|AllPartsMoving)))

(event Custom|P3_HeadLeftCheck
  (params (TimerId :type String))
  ;[1 1 1] 阶段3_1_张开双眼，并左右转头
  ;;[1 1 1] 循环检测左转头
  (if (Variables|/Script/OldMan.OldManBossHead|GetIsLeftEarRight (Variables|TargetActor|GetBossHead))
    (Variables|Default|SetP3_Left true)
    (Class|MonoManager|ClearTimer (Class|MonoManager|GetMonoManager) "P3_HeadLeftCheck")
    ;;[1 1 1] P3_左转头回正
    (Class|OldManTipLight|SwitchCanMoveMat (Variables|TargetActor|GetTipLight) false)
    (Class|OldManBossHead|SetPartActive (Variables|TargetActor|GetBossHead) "TurnHeadLeft" false)
    (Class|OldManBossHead|LeftEarBack (Variables|TargetActor|GetBossHead))
    (Class|MonoManager|SetIntervalwithId (Class|MonoManager|GetMonoManager) 0.5 "P3_TurnHeadLeftCheck" (delegate Custom|P3_HeadLeftBack))))

(event Custom|P3_HeadRightBack
  (params (TimerId :type String))
  ;[1 1 1] 阶段3_1_张开双眼，并左右转头
  ;;[1 1 1] P3_右转头回正
  (if (Variables|/Script/OldMan.OldManBossHead|GetRightEarBackCompelete (Variables|TargetActor|GetBossHead))
    (Class|MonoManager|ClearTimer (Class|MonoManager|GetMonoManager) "P3_TurnHeadRightCheck")
    (Class|OldManTipLight|SwitchCanMoveMat (Variables|TargetActor|GetTipLight) true)
    (Development|PrintString "PlayerCompelete")))

(event Custom|P2_HeadRightCheck2
  (params (TimerId :type String))
  ;[1 1 1] 阶段2_2_右转头
  (if (Variables|/Script/OldMan.OldManBossHead|GetRightEarBackCompelete (Variables|TargetActor|GetBossHead))
    (Class|MonoManager|ClearTimer (Class|MonoManager|GetMonoManager) "P2_TurnHeadRightCheck")
    (Class|OldManBossHead|SetPartActive (Variables|TargetActor|GetBossHead) "TurnHeadRight" true)
    (Class|OldManBossHead|RightEarBlink (Variables|TargetActor|GetBossHead))
    (Class|OldManTipLight|SwitchCanMoveMat (Variables|TargetActor|GetTipLight) true)
    (EventDispatchers|BindEventtoOnSoundFinished (Class|AudioManager|GetAudioManager) (delegate Custom|P2_2_CountTimeCompelete))
    ;;[1 1 1] 阶段2地板生成
    (Development|PrintString "阶段2地板生成")
    ;;[1 1 1] 倒计时音频
    (Class|AudioManager|PlaySound (Class|AudioManager|GetAudioManager) "Test7" 0 "0, 0, 0" 0.0 0.0 1.0)
    (Development|PrintString "倒计时音频")))

(event Custom|P1_RightEyebrow_AudioCompelete
  (params (SoundID :type Name))
  ;[1 1 1] 阶段1_2_张开右眼
  (EventDispatchers|UnbindEventfromOnSoundFinished (Class|AudioManager|GetAudioManager) (delegate Custom|P1_RightEyebrow_AudioCompelete))
  (Class|OldManBossHead|SetPartActive (Variables|TargetActor|GetBossHead) "RightEyebrow" true)
  (Class|OldManBossHead|RightEyebrowBlink (Variables|TargetActor|GetBossHead))
  (Class|OldManTipLight|SwitchCanMoveMat (Variables|TargetActor|GetTipLight) true)
  (EventDispatchers|BindEventtoOnSoundFinished (Class|AudioManager|GetAudioManager) (delegate Custom|P1_RightEyebrow_CountDownCompelete))
  ;;[1 1 1] 倒计时音频
  (Class|AudioManager|PlaySound (Class|AudioManager|GetAudioManager) "Test5" 0 "0, 0, 0" 0.0 0.0 1.0)
  (Development|PrintString "倒计时音频"))

(event Custom|P1_Chin_AudioCompelete
  (params (SoundID :type Name))
  ;[1 1 1] 阶段1_3_张开下巴
  (EventDispatchers|UnbindEventfromOnSoundFinished (Class|AudioManager|GetAudioManager) (delegate Custom|P1_Chin_AudioCompelete))
  (Class|OldManBossHead|SetPartActive (Variables|TargetActor|GetBossHead) "Chin" true)
  (Class|OldManBossHead|ChinBlink (Variables|TargetActor|GetBossHead))
  (Class|OldManTipLight|SwitchCanMoveMat (Variables|TargetActor|GetTipLight) true)
  (EventDispatchers|BindEventtoOnSoundFinished (Class|AudioManager|GetAudioManager) (delegate Custom|P1_Chin_CountDownCompelete))
  ;;[1 1 1] 倒计时音频
  (Class|AudioManager|PlaySound (Class|AudioManager|GetAudioManager) "Test5" 0 "0, 0, 0" 0.0 0.0 1.0)
  (Development|PrintString "倒计时音频"))

(event Custom|P1_RightEyebrow_CountDownCompelete
  (params (SoundID :type Name))
  ;[1 1 1] 阶段1_2_张开右眼
  (EventDispatchers|UnbindEventfromOnSoundFinished (Class|AudioManager|GetAudioManager) (delegate Custom|P1_RightEyebrow_CountDownCompelete))
  (Class|OldManBossHead|SetPartActive (Variables|TargetActor|GetBossHead) "RightEyebrow" false)
  (Class|OldManTipLight|SwitchCanMoveMat (Variables|TargetActor|GetTipLight) false)
  (Class|OldManMobileCamera|BeginScanWithoutParm (Variables|TargetActor|GetScanLight))
  (Class|MonoManager|SetIntervalwithId (Class|MonoManager|GetMonoManager) 1.0 "P1_OpenRightEyebrowScan" (delegate Custom|P1_RightEyebrow_ScanCompelete)))

(event Custom|P1_RightEyebrow_ScanCompelete
  (params (TimerId :type String))
  ;[1 1 1] 阶段1_2_张开右眼
  (Class|MonoManager|ClearTimer (Class|MonoManager|GetMonoManager) "P1_OpenRightEyebrowScan")
  (Class|OldManMobileCamera|CloseLight (Variables|TargetActor|GetScanLight))
  (if (Variables|/Script/OldMan.OldManBossHead|GetIsRightEyebrowOpen (Variables|TargetActor|GetBossHead))
    ;;[1 1 1] 环境光提示
    (Development|PrintString "环境光提示")
    (Class|OldManBossHead|RightEyebrowClose (Variables|TargetActor|GetBossHead))
    ;[1 1 1] 阶段1_3_张开下巴
    (EventDispatchers|BindEventtoOnSoundFinished (Class|AudioManager|GetAudioManager) (delegate Custom|P1_Chin_AudioCompelete))
    ;;[1 1 1] 播放请张开下巴音频
    (Class|AudioManager|PlaySound (Class|AudioManager|GetAudioManager) "TestYveYin" 0 "0, 0, 0" 0.0 0.0 1.0)
    (Development|PrintString "播放请张开下巴音频")
    (Class|OldManTipLight|SwitchOperationMat (Variables|TargetActor|GetTipLight) "Chin")
    (else
      (Development|PrintString "环境光提示")
      (Class|OldManBossHead|RightEyebrowClose (Variables|TargetActor|GetBossHead))
      (Class|OldManBossHead|SetPartActive (Variables|TargetActor|GetBossHead) "RightEyebrow" true)
      (Class|OldManBossHead|RightEyebrowBlink (Variables|TargetActor|GetBossHead))
      (Class|OldManTipLight|SwitchCanMoveMat (Variables|TargetActor|GetTipLight) true)
      (EventDispatchers|BindEventtoOnSoundFinished (Class|AudioManager|GetAudioManager) (delegate Custom|P1_RightEyebrow_CountDownCompelete))
      ;;[1 1 1] 倒计时音频
      (Class|AudioManager|PlaySound (Class|AudioManager|GetAudioManager) "Test5" 0 "0, 0, 0" 0.0 0.0 1.0)
      (Development|PrintString "倒计时音频"))))

(event Custom|P1_Chin_CountDownCompelete
  (params (SoundID :type Name))
  ;[1 1 1] 阶段1_3_张开下巴
  (EventDispatchers|UnbindEventfromOnSoundFinished (Class|AudioManager|GetAudioManager) (delegate Custom|P1_Chin_CountDownCompelete))
  (Class|OldManBossHead|SetPartActive (Variables|TargetActor|GetBossHead) "Chin" false)
  (Class|OldManTipLight|SwitchCanMoveMat (Variables|TargetActor|GetTipLight) false)
  (Class|OldManMobileCamera|BeginScanWithoutParm (Variables|TargetActor|GetScanLight))
  (Class|MonoManager|SetIntervalwithId (Class|MonoManager|GetMonoManager) 1.0 "P1_OpenChinScan" (delegate Custom|P1_Chin_ScanCompelete)))

(event Custom|P1_LeftEyebrow_CountDownCompelete
  (params (SoundID :type Name))
  ;[1 1 1] 阶段1_1_张开左眼
  (EventDispatchers|UnbindEventfromOnSoundFinished (Class|AudioManager|GetAudioManager) (delegate Custom|P1_LeftEyebrow_CountDownCompelete))
  (Class|OldManBossHead|SetPartActive (Variables|TargetActor|GetBossHead) "LeftEyebrow" false)
  (Class|OldManTipLight|SwitchCanMoveMat (Variables|TargetActor|GetTipLight) false)
  (Class|OldManMobileCamera|BeginScanWithoutParm (Variables|TargetActor|GetScanLight))
  (Class|MonoManager|SetIntervalwithId (Class|MonoManager|GetMonoManager) 1.0 "P1_OpenLeftEyebrowScan" (delegate Custom|P1_LeftEyebrow_ScanCompelete)))

(event Custom|P2_1_TurnHeadLeftAudioCompelete
  (params (SoundID :type Name))
  ;[1 1 1] 阶段2_1_左转头
  (EventDispatchers|UnbindEventfromOnSoundFinished (Class|AudioManager|GetAudioManager) (delegate Custom|P2_1_TurnHeadLeftAudioCompelete))
  (Class|OldManBossHead|SetPartActive (Variables|TargetActor|GetBossHead) "TurnHeadLeft" true)
  (Class|OldManBossHead|LeftEarBlink (Variables|TargetActor|GetBossHead))
  (Class|OldManTipLight|SwitchCanMoveMat (Variables|TargetActor|GetTipLight) true)
  (EventDispatchers|BindEventtoOnSoundFinished (Class|AudioManager|GetAudioManager) (delegate Custom|P2_1HeadLeftCountTimeCompelete))
  ;;[1 1 1] 阶段2地板生成
  (Development|PrintString "阶段2地板生成")
  ;;[1 1 1] 倒计时音频
  (Class|AudioManager|PlaySound (Class|AudioManager|GetAudioManager) "Test7" 0 "0, 0, 0" 0.0 0.0 1.0)
  (Development|PrintString "倒计时音频"))

(event Custom|P2_1HeadLeftCountTimeCompelete
  (params (SoundID :type Name))
  ;[1 1 1] 阶段2_1_左转头
  (EventDispatchers|UnbindEventfromOnSoundFinished (Class|AudioManager|GetAudioManager) (delegate Custom|P2_1HeadLeftCountTimeCompelete))
  (Class|OldManBossHead|SetPartActive (Variables|TargetActor|GetBossHead) "TurnHeadLeft" false)
  (Class|OldManTipLight|SwitchCanMoveMat (Variables|TargetActor|GetTipLight) false)
  (Class|OldManMobileCamera|BeginScanWithoutParm (Variables|TargetActor|GetScanLight))
  (Class|MonoManager|SetIntervalwithId (Class|MonoManager|GetMonoManager) 1.0 "P2_TurnHeadLeftScan" (delegate Custom|P2_1_HeadLeftScanCompelete)))

(event Custom|P2_1_HeadLeftScanCompelete
  (params (TimerId :type String))
  ;[1 1 1] 阶段2_1_左转头
  (Class|MonoManager|ClearTimer (Class|MonoManager|GetMonoManager) "P2_TurnHeadLeftScan")
  (Class|OldManMobileCamera|CloseLight (Variables|TargetActor|GetScanLight))
  (if (Variables|/Script/OldMan.OldManBossHead|GetIsLeftEarRight (Variables|TargetActor|GetBossHead))
    ;;[1 1 1] 环境光提示
    (Development|PrintString "环境光提示")
    (Class|OldManBossHead|LeftEarBack (Variables|TargetActor|GetBossHead))
    (Class|MonoManager|SetIntervalwithId (Class|MonoManager|GetMonoManager) 0.5 "P2_TurnHeadLeftCheck" (delegate Custom|P2_1_Check))
    (else
      (Development|PrintString "环境光提示")
      (Class|OldManBossHead|LeftEarBack (Variables|TargetActor|GetBossHead))
      (Class|MonoManager|SetIntervalwithId (Class|MonoManager|GetMonoManager) 0.5 "P2_TurnHeadLeftCheck" (delegate Custom|P2_1_Check2)))))

(event Custom|P3_HeadLeftBack
  (params (TimerId :type String))
  ;[1 1 1] 阶段3_1_张开双眼，并左右转头
  ;;[1 1 1] P3_左转头回正
  (if (Variables|/Script/OldMan.OldManBossHead|GetLeftEarBackCompelete (Variables|TargetActor|GetBossHead))
    (Class|MonoManager|ClearTimer (Class|MonoManager|GetMonoManager) "P3_TurnHeadLeftCheck")
    (Class|OldManTipLight|SwitchCanMoveMat (Variables|TargetActor|GetTipLight) true)
    ;;[1 1 1] 循环检测右转头
    (Class|OldManBossHead|SetPartActive (Variables|TargetActor|GetBossHead) "TurnHeadRight" true)
    (Class|OldManTipLight|SwitchOperationMat (Variables|TargetActor|GetTipLight) "TurnHeadRight")
    (Class|MonoManager|SetIntervalwithId (Class|MonoManager|GetMonoManager) 0.5 "P3_HeadRightCheck" (delegate Custom|P3_HeadRightCheck))))

(event Custom|P3_HeadRightCheck
  (params (TimerId :type String))
  ;[1 1 1] 阶段3_1_张开双眼，并左右转头
  ;;[1 1 1] 循环检测右转头
  (if (Variables|/Script/OldMan.OldManBossHead|GetIsRightEarRight (Variables|TargetActor|GetBossHead))
    (Variables|Default|SetP3_Right true)
    (Class|MonoManager|ClearTimer (Class|MonoManager|GetMonoManager) "P3_HeadRightCheck")
    ;;[1 1 1] P3_右转头回正
    (Class|OldManTipLight|SwitchCanMoveMat (Variables|TargetActor|GetTipLight) false)
    (Class|OldManBossHead|SetPartActive (Variables|TargetActor|GetBossHead) "TurnHeadRight" false)
    (Class|OldManBossHead|RightEarBack (Variables|TargetActor|GetBossHead))
    (Class|MonoManager|SetIntervalwithId (Class|MonoManager|GetMonoManager) 0.5 "P3_TurnHeadRightCheck" (delegate Custom|P3_HeadRightBack))))

(event Custom|P1_LeftEyebrow_ScanCompelete
  (params (TimerId :type String))
  ;[1 1 1] 阶段1_1_张开左眼
  (Class|MonoManager|ClearTimer (Class|MonoManager|GetMonoManager) "P1_OpenLeftEyebrowScan")
  (Class|OldManMobileCamera|CloseLight (Variables|TargetActor|GetScanLight))
  (if (Variables|/Script/OldMan.OldManBossHead|GetIsLeftEyebrowOpen (Variables|TargetActor|GetBossHead))
    ;;[1 1 1] 环境光提示
    (Development|PrintString "环境光提示")
    (Class|OldManBossHead|LeftEyebrowClose (Variables|TargetActor|GetBossHead))
    ;[1 1 1] 阶段1_2_张开右眼
    (EventDispatchers|BindEventtoOnSoundFinished (Class|AudioManager|GetAudioManager) (delegate Custom|P1_RightEyebrow_AudioCompelete))
    ;;[1 1 1] 播放请张开右眼音频
    (Class|AudioManager|PlaySound (Class|AudioManager|GetAudioManager) "TestYveYin" 0 "0, 0, 0" 0.0 0.0 1.0)
    (Development|PrintString "播放请张开右眼音频")
    (Class|OldManTipLight|SwitchOperationMat (Variables|TargetActor|GetTipLight) "RightEyebrow")
    (else
      (Development|PrintString "环境光提示")
      (Class|OldManBossHead|LeftEyebrowClose (Variables|TargetActor|GetBossHead))
      (Class|OldManBossHead|SetPartActive (Variables|TargetActor|GetBossHead) "LeftEyebrow" true)
      (Class|OldManBossHead|LeftEyebrowBlink (Variables|TargetActor|GetBossHead))
      (Class|OldManTipLight|SwitchCanMoveMat (Variables|TargetActor|GetTipLight) true)
      (EventDispatchers|BindEventtoOnSoundFinished (Class|AudioManager|GetAudioManager) (delegate Custom|P1_LeftEyebrow_CountDownCompelete))
      ;;[1 1 1] 阶段1地板随机生成
      (Development|PrintString "阶段1地板随机生成")
      ;;[1 1 1] 倒计时音频
      (Class|AudioManager|PlaySound (Class|AudioManager|GetAudioManager) "Test5" 0 "0, 0, 0" 0.0 0.0 1.0)
      (Development|PrintString "倒计时音频"))))

(event Custom|P3_CountTimeCompelete
  (params (SoundID :type Name))
  ;[1 1 1] 阶段3_1_张开双眼，并左右转头
  (EventDispatchers|UnbindEventfromOnSoundFinished (Class|AudioManager|GetAudioManager) (delegate Custom|P3_CountTimeCompelete))
  (Class|OldManTipLight|SwitchCanMoveMat (Variables|TargetActor|GetTipLight) false)
  (Class|OldManMobileCamera|CloseLight (Variables|TargetActor|GetScanLight))
  (Class|OldManBossHead|SetAllPartActive (Variables|TargetActor|GetBossHead) false)
  (if (and (and (Variables|Default|GetP3_Left) (Variables|Default|GetP3_Right)) (and (Variables|/Script/OldMan.OldManBossHead|GetIsLeftEyebrowOpen (Variables|TargetActor|GetBossHead)) (Variables|/Script/OldMan.OldManBossHead|GetIsRightEyebrowOpen (Variables|TargetActor|GetBossHead))))
    ;;[1 1 1] 环境光提示
    (Development|PrintString "环境光提示")
    (Class|OldManBossHead|SetAllPartBack (Variables|TargetActor|GetBossHead))
    (Development|PrintString "Compelete")
    (else
      (Development|PrintString "环境光提示")
      (Class|OldManBossHead|SetAllPartBack (Variables|TargetActor|GetBossHead))
      (Class|OldManBossHead|SetPartActive (Variables|TargetActor|GetBossHead) "Eyebrow" true)
      (Class|OldManTipLight|SwitchOperationMat (Variables|TargetActor|GetTipLight) "Eyebrow")
      (Class|OldManBossHead|LeftEarBlink (Variables|TargetActor|GetBossHead))
      (Class|OldManBossHead|RightEarBlink (Variables|TargetActor|GetBossHead))
      (Class|OldManTipLight|SwitchCanMoveMat (Variables|TargetActor|GetTipLight) true)
      (Class|OldManMobileCamera|BeginScanWithoutParm (Variables|TargetActor|GetScanLight))
      (EventDispatchers|BindEventtoOnSoundFinished (Class|AudioManager|GetAudioManager) (delegate Custom|P3_CountTimeCompelete))
      ;;[1 1 1] 倒计时
      (Class|AudioManager|PlaySound (Class|AudioManager|GetAudioManager) "Test30" 0 "0, 0, 0" 0.0 0.0 1.0)
      (Development|PrintString "倒计时")
      (Class|MonoManager|SetIntervalwithId (Class|MonoManager|GetMonoManager) 0.5 "CheckMoving" (delegate Custom|AllPartsMoving)))))

(event Custom|P2_1_Check2
  (params (TimerId :type String))
  ;[1 1 1] 阶段2_1_左转头
  (if (Variables|/Script/OldMan.OldManBossHead|GetLeftEarBackCompelete (Variables|TargetActor|GetBossHead))
    (Class|MonoManager|ClearTimer (Class|MonoManager|GetMonoManager) "P2_TurnHeadLeftCheck")
    (Class|OldManBossHead|SetPartActive (Variables|TargetActor|GetBossHead) "TurnHeadLeft" true)
    (Class|OldManBossHead|LeftEarBlink (Variables|TargetActor|GetBossHead))
    (Class|OldManTipLight|SwitchCanMoveMat (Variables|TargetActor|GetTipLight) true)
    (EventDispatchers|BindEventtoOnSoundFinished (Class|AudioManager|GetAudioManager) (delegate Custom|P2_1HeadLeftCountTimeCompelete))
    ;;[1 1 1] 阶段2地板生成
    (Development|PrintString "阶段2地板生成")
    ;;[1 1 1] 倒计时音频
    (Class|AudioManager|PlaySound (Class|AudioManager|GetAudioManager) "Test7" 0 "0, 0, 0" 0.0 0.0 1.0)
    (Development|PrintString "倒计时音频")))

(event Custom|P3_EyebrowCheck
  (params (TimerId :type String))
  (bind _bosshead (Variables|TargetActor|GetBossHead))
  ;[1 1 1] 阶段3_1_张开双眼，并左右转头
  ;;[1 1 1] 循环检测是否张开双眼
  (if (and (Variables|/Script/OldMan.OldManBossHead|GetIsRightEyebrowOpen _bosshead) (Variables|/Script/OldMan.OldManBossHead|GetIsLeftEyebrowOpen _bosshead))
    (Class|MonoManager|ClearTimer (Class|MonoManager|GetMonoManager) "P3_EyebrowCheck")
    ;;[1 1 1] 循环检测左转头
    (Class|OldManBossHead|SetPartActive (Variables|TargetActor|GetBossHead) "TurnHeadLeft" true)
    (Class|OldManTipLight|SwitchOperationMat (Variables|TargetActor|GetTipLight) "TurnHeadLeft")
    (Class|MonoManager|SetIntervalwithId (Class|MonoManager|GetMonoManager) 0.5 "P3_HeadLeftCheck" (delegate Custom|P3_HeadLeftCheck))))

(event Custom|AllPartsMoving
  (params (TimerId :type String))
  ;[1 1 1] 阶段3_1_张开双眼，并左右转头
  (if (Variables|/Script/OldMan.OldManBossHead|GetAllPartsMovingEnd (Variables|TargetActor|GetBossHead))
    (Variables|Default|SetP3_Left true)
    (Class|MonoManager|ClearTimer (Class|MonoManager|GetMonoManager) "CheckMoving")
    ;;[1 1 1] 循环检测是否张开双眼
    (Class|MonoManager|SetIntervalwithId (Class|MonoManager|GetMonoManager) 0.5 "P3_EyebrowCheck" (delegate Custom|P3_EyebrowCheck))))

(event Custom|P2_1_Check
  (params (TimerId :type String))
  ;[1 1 1] 阶段2_1_左转头
  (if (Variables|/Script/OldMan.OldManBossHead|GetLeftEarBackCompelete (Variables|TargetActor|GetBossHead))
    (Class|MonoManager|ClearTimer (Class|MonoManager|GetMonoManager) "P2_TurnHeadLeftCheck")
    ;[1 1 1] 阶段2_2_右转头
    (EventDispatchers|BindEventtoOnSoundFinished (Class|AudioManager|GetAudioManager) (delegate Custom|P2_2_HeadRightAudioCompelete))
    ;;[1 1 1] 播放请右转头
    (Class|AudioManager|PlaySound (Class|AudioManager|GetAudioManager) "TestYveYin" 0 "0, 0, 0" 0.0 0.0 1.0)
    (Development|PrintString "播放请右转头")
    (Class|OldManTipLight|SwitchOperationMat (Variables|TargetActor|GetTipLight) "TurnHeadRight")))

(event Custom|P1_Chin_ScanCompelete
  (params (TimerId :type String))
  ;[1 1 1] 阶段1_3_张开下巴
  (Class|MonoManager|ClearTimer (Class|MonoManager|GetMonoManager) "P1_OpenChinScan")
  (Class|OldManMobileCamera|CloseLight (Variables|TargetActor|GetScanLight))
  (if (Variables|/Script/OldMan.OldManBossHead|GetIsChinOpen (Variables|TargetActor|GetBossHead))
    ;;[1 1 1] 环境光提示
    (Development|PrintString "环境光提示")
    (Class|OldManBossHead|ChinClose (Variables|TargetActor|GetBossHead))
    ;[1 1 1] 滑索升起
    (Development|PrintString "滑索升起")
    (Class|OldManBossHead|SetAllPartActive (Variables|TargetActor|GetBossHead) false)
    (Class|OldManBossHead|SetAllPartBack (Variables|TargetActor|GetBossHead))
    ;[1 1 1] 阶段2_1_左转头
    (EventDispatchers|BindEventtoOnSoundFinished (Class|AudioManager|GetAudioManager) (delegate Custom|P2_1_TurnHeadLeftAudioCompelete))
    ;;[1 1 1] 播放请左转头
    (Class|AudioManager|PlaySound (Class|AudioManager|GetAudioManager) "TestYveYin" 0 "0, 0, 0" 0.0 0.0 1.0)
    (Development|PrintString "播放请左转头")
    (Class|OldManTipLight|SwitchOperationMat (Variables|TargetActor|GetTipLight) "TurnHeadLeft")
    (else
      (Development|PrintString "环境光提示")
      (Class|OldManBossHead|ChinClose (Variables|TargetActor|GetBossHead))
      (Class|OldManBossHead|SetPartActive (Variables|TargetActor|GetBossHead) "Chin" true)
      (Class|OldManBossHead|ChinBlink (Variables|TargetActor|GetBossHead))
      (Class|OldManTipLight|SwitchCanMoveMat (Variables|TargetActor|GetTipLight) true)
      (EventDispatchers|BindEventtoOnSoundFinished (Class|AudioManager|GetAudioManager) (delegate Custom|P1_Chin_CountDownCompelete))
      ;;[1 1 1] 倒计时音频
      (Class|AudioManager|PlaySound (Class|AudioManager|GetAudioManager) "Test5" 0 "0, 0, 0" 0.0 0.0 1.0)
      (Development|PrintString "倒计时音频"))))

(event Custom|P2_HeadRightCheck
  (params (TimerId :type String))
  ;[1 1 1] 阶段2_2_右转头
  (if (Variables|/Script/OldMan.OldManBossHead|GetRightEarBackCompelete (Variables|TargetActor|GetBossHead))
    (Class|MonoManager|ClearTimer (Class|MonoManager|GetMonoManager) "P2_TurnHeadRightCheck")
    (Class|OldManBossHead|SetAllPartActive (Variables|TargetActor|GetBossHead) false)
    (Class|OldManBossHead|SetAllPartBack (Variables|TargetActor|GetBossHead))
    ;[1 1 1] 阶段3_1_张开双眼，并左右转头
    ;;[1 1 1] 敌人预留
    (Development|PrintString "敌人预留")
    (EventDispatchers|BindEventtoOnSoundFinished (Class|AudioManager|GetAudioManager) (delegate Custom|P3_Eyebrow))
    ;;[1 1 1] 播放请张开双眼、并左右转头
    (Class|AudioManager|PlaySound (Class|AudioManager|GetAudioManager) "TestYveYin" 0 "0, 0, 0" 0.0 0.0 1.0)
    (Development|PrintString "播放请张开双眼、并左右转头")
    (Class|OldManTipLight|SwitchOperationMat (Variables|TargetActor|GetTipLight) "Eyebrow")))

(event Custom|P2_2_HeadRightAudioCompelete
  (params (SoundID :type Name))
  ;[1 1 1] 阶段2_2_右转头
  (EventDispatchers|UnbindEventfromOnSoundFinished (Class|AudioManager|GetAudioManager) (delegate Custom|P2_2_HeadRightAudioCompelete))
  (Class|OldManBossHead|SetPartActive (Variables|TargetActor|GetBossHead) "TurnHeadRight" true)
  (Class|OldManBossHead|RightEarBlink (Variables|TargetActor|GetBossHead))
  (Class|OldManTipLight|SwitchCanMoveMat (Variables|TargetActor|GetTipLight) true)
  (EventDispatchers|BindEventtoOnSoundFinished (Class|AudioManager|GetAudioManager) (delegate Custom|P2_2_CountTimeCompelete))
  ;;[1 1 1] 阶段2地板生成
  (Development|PrintString "阶段2地板生成")
  ;;[1 1 1] 倒计时音频
  (Class|AudioManager|PlaySound (Class|AudioManager|GetAudioManager) "Test7" 0 "0, 0, 0" 0.0 0.0 1.0)
  (Development|PrintString "倒计时音频"))

(event Custom|P2_2_CountTimeCompelete
  (params (SoundID :type Name))
  ;[1 1 1] 阶段2_2_右转头
  (EventDispatchers|UnbindEventfromOnSoundFinished (Class|AudioManager|GetAudioManager) (delegate Custom|P2_2_CountTimeCompelete))
  (Class|OldManBossHead|SetPartActive (Variables|TargetActor|GetBossHead) "TurnHeadRight" false)
  (Class|OldManTipLight|SwitchCanMoveMat (Variables|TargetActor|GetTipLight) false)
  (Class|OldManMobileCamera|BeginScanWithoutParm (Variables|TargetActor|GetScanLight))
  (Class|MonoManager|SetIntervalwithId (Class|MonoManager|GetMonoManager) 1.0 "P2_TurnHeadRightScan" (delegate Custom|P2_2_HeadRightScanCompelete)))

(event Custom|P2_2_HeadRightScanCompelete
  (params (TimerId :type String))
  ;[1 1 1] 阶段2_2_右转头
  (Class|MonoManager|ClearTimer (Class|MonoManager|GetMonoManager) "P2_TurnHeadRightScan")
  (Class|OldManMobileCamera|CloseLight (Variables|TargetActor|GetScanLight))
  (if (Variables|/Script/OldMan.OldManBossHead|GetIsRightEarRight (Variables|TargetActor|GetBossHead))
    ;;[1 1 1] 环境光提示
    (Development|PrintString "环境光提示")
    (Class|OldManBossHead|SetAllPartBack (Variables|TargetActor|GetBossHead))
    (Class|MonoManager|SetIntervalwithId (Class|MonoManager|GetMonoManager) 0.5 "P2_TurnHeadRightCheck" (delegate Custom|P2_HeadRightCheck))
    (else
      (Development|PrintString "环境光提示")
      (Class|OldManBossHead|RightEarBack (Variables|TargetActor|GetBossHead))
      (Class|MonoManager|SetIntervalwithId (Class|MonoManager|GetMonoManager) 0.5 "P2_TurnHeadRightCheck" (delegate Custom|P2_HeadRightCheck2)))))

(event EventBeginPlay
  ;[1 1 1] 初始化
  (Class|OldManBossHead|SetAllPartActive (Variables|TargetActor|GetBossHead) false)
  (Class|OldManBossHead|SetAllPartBack (Variables|TargetActor|GetBossHead))
  (Class|OldManBossHead|UpdateData (Variables|TargetActor|GetBossHead))
  (Class|OldManTipLight|SwitchCanMoveMat (Variables|TargetActor|GetTipLight) true)
  (Class|OldManTipLight|SwitchOperationMat (Variables|TargetActor|GetTipLight) "Eyebrow")
  (Class|OldManMobileCamera|CloseLight (Variables|TargetActor|GetScanLight))
  ;;[1 1 1] 地板预留
  (Development|PrintString "地板预留"))

(event Collision|EventActorBeginOverlap
  (params (OtherActor :type Actor%20Object%20Reference)))

(event EventTick
  (params (DeltaSeconds :type Float%20%28single-precision%29)))

(fn ConstructionScript)