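; Boss-area scan light controller that switches a referenced scan drone and its light between open and closed states.
; Open opens ScanLight, shows BPScanDrone with its tick and collision disabled, and plays a level sequence.
; Close closes the light and restores the BeginPlay drone state, hidden yet ticking and collidable, without stopping the sequence.
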(event EventBeginPlay
  (bind _bp_scandrone (Variables|Default|GetBP_ScanDrone))
  (Actor|Tick|SetActorTickEnabled _bp_scandrone true)
  (Collision|SetActorEnableCollision _bp_scandrone true)
  (Rendering|SetActorHiddenInGame _bp_scandrone true))

(event Collision|EventActorBeginOverlap
  (params (OtherActor :type Actor%20Object%20Reference)))

(event EventTick
  (params (DeltaSeconds :type Float%20%28single-precision%29)))

(event EventOpen
  (bind _bp_scandrone (Variables|Default|GetBP_ScanDrone))
  (Default|Open (Variables|Default|GetScanLight))
  (Actor|Tick|SetActorTickEnabled _bp_scandrone)
  (Collision|SetActorEnableCollision _bp_scandrone false)
  (Rendering|SetActorHiddenInGame _bp_scandrone false)
  (Sequencer|Player|Play (Variables|/Script/LevelSequence.LevelSequenceActor|GetSequencePlayer (Variables|Default|GetSequencer)) :!class /Script/MovieScene.MovieSceneSequencePlayer))

(event EventClose
  (bind _bp_scandrone (Variables|Default|GetBP_ScanDrone))
  (Default|Close (Variables|Default|GetScanLight))
  (Actor|Tick|SetActorTickEnabled _bp_scandrone true)
  (Collision|SetActorEnableCollision _bp_scandrone true)
  (Rendering|SetActorHiddenInGame _bp_scandrone true))

(fn ConstructionScript)