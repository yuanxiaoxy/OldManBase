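; BP_Trail_Showcase is a demo actor that previews a dash trail effect in motion.
; The construction script assigns the InAsset variable to the Dash effect component.
; From BeginPlay, a timeline lerps Sphere between the world locations of Sphere1 and Sphere2.
; When the timeline finishes, a short delay precedes a reset of Dash and a replay from the start, looping the showcase.
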(event EventBeginPlay
  (bind _newtrack_0 (Timeline|Timeline_0 PlayFromStart)
    (:Update
      (Transformation|SetWorldLocation (Variables|Default|GetSphere) (Math|Vector|Lerp(Vector) (Transformation|GetWorldLocation (Variables|Default|GetSphere1)) (Transformation|GetWorldLocation (Variables|Default|GetSphere2)) _newtrack_0) false false))
    (:Finished
      (Utilities|FlowControl|Delay 0.1)
      (Components|Activation|SetActive (Variables|Default|Getdash) true true)
      (Timeline|Timeline_0 PlayFromStart))))

(fn ConstructionScript
  (Class|NiagaraComponent|SetAsset (Variables|Default|Getdash) (Variables|Default|GetIn%20Asset) true))