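; Boss door that powers up when the player enters and opens through a drag interaction.
; Entry fades in three lights and runs a timed scan effect, then swaps the upper door material and enables dragging; exit resets these.
; Dragging drives a material Time parameter through a reversible timeline, revealing the active stick and unlocking opening upon completion.
; A downward view direction then opens both door halves through timeline lerps, with a separate timeline for closing.
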(event Custom|CloseDoor
  (bind _step (Timeline|时间轴 Play)
    (:Update
      (Transformation|SetRelativeLocation (Variables|Default|GetSM_UpDoor) (Math|Vector|Lerp(Vector) (Variables|Default|GetUpDoorOpenPos) (Variables|Default|GetUpDoorInitPos) _step) false false)
      (Transformation|SetRelativeLocation (Variables|Default|GetSM_DownDoor) (Math|Vector|Lerp(Vector) (Variables|Default|GetDownDoorOpennPos) (Variables|Default|GetDownDoorInitPos) _step) false false))))

(event Custom|OnPlayerEnter
  (Development|PrintString "顺序亮灯")
  (bind _新建轨道_0 (Timeline|灯亮 PlayFromStart)
    (:Update
      (Rendering|Components|Light|SetIntensity (Variables|Default|GetPointLight_Left) (* (Variables|Default|GetIntensity_Left) _新建轨道_0))
      (Rendering|Components|Light|SetIntensity (Variables|Default|GetPointLight_Right) (* _新建轨道_0 (Variables|Default|GetIntensity_Right)))
      (Rendering|Components|Light|SetIntensity (Variables|Default|GetPointLight_Mid) (* (Variables|Default|GetIntensity_Mid) _新建轨道_0)))
    (:Finished
      (Components|Activation|Activate (Variables|Default|GetNS_BossDoor_Line2) false)
      (Class|MonoManager|SetTimeoutSimplewithId (Class|MonoManager|GetMonoManager) 1.0 "BossDoor" (delegate Custom|扫描结束)))))

(event Custom|扫描结束
  (Class|MonoManager|ClearTimer (Class|MonoManager|GetMonoManager) "BossDoor")
  (Components|Activation|Deactivate (Variables|Default|GetNS_BossDoor_Line2))
  (Rendering|Material|SetMaterial (Variables|Default|GetSM_UpDoor) 1 (Variables|Default|GetTarget))
  (Variables|Default|SetCanDrag true))

(event Custom|OnPlayerExit
  (Development|PrintString "若灯光开启则关闭所有灯光")
  (Rendering|Components|Light|SetIntensity (Variables|Default|GetPointLight_Left) 0.0)
  (Rendering|Components|Light|SetIntensity (Variables|Default|GetPointLight_Mid) 0.0)
  (Components|Activation|Deactivate (Variables|Default|GetNS_BossDoor_Line2))
  (Rendering|Components|Light|SetIntensity (Variables|Default|GetPointLight_Right) 0.0)
  (Rendering|Material|SetMaterial (Variables|Default|GetSM_UpDoor) 1 (Variables|Default|GetInit))
  (Variables|Default|SetCanDrag false))

(event Custom|OpenDoor
  (bind _step (Timeline|OpenCloseDoorTimeLine Play)
    (:Update
      (Transformation|SetRelativeLocation (Variables|Default|GetSM_UpDoor) (Math|Vector|Lerp(Vector) (Variables|Default|GetUpDoorInitPos) (Variables|Default|GetUpDoorOpenPos) _step) false false)
      (Transformation|SetRelativeLocation (Variables|Default|GetSM_DownDoor) (Math|Vector|Lerp(Vector) (Variables|Default|GetDownDoorInitPos) (Variables|Default|GetDownDoorOpennPos) _step) false false))))

(event EventBeginPlay
  (Rendering|SetVisibility (Variables|Default|GetSM_Stick_Active) false false)
  (Rendering|Components|Light|SetIntensity (Variables|Default|GetPointLight_Left) 0.0)
  (Rendering|Components|Light|SetIntensity (Variables|Default|GetPointLight_Right) 0.0)
  (Rendering|Components|Light|SetIntensity (Variables|Default|GetPointLight_Mid) 0.0)
  (Components|Activation|Deactivate (Variables|Default|GetNS_BossDoor_Line2))
  (Variables|Default|SetInit (Rendering|Material|GetMaterial (Variables|Default|GetSM_Stick_Active) 1))
  (Actor|Tick|SetActorTickEnabled false))

(event Collision|EventActorBeginOverlap
  (params (OtherActor :type Actor%20Object%20Reference)))

(event EventHandleMouseData
  (params (ViewDirection :type Vector%20%28by%20ref%29 :default "0, 0, 0") (Intensity :type Float%20%28single-precision%29))
  (if (Variables|Default|GetCanOpen)
    (if (<= (.z ViewDirection) -0.5)
      (CallFunction|OpenDoor))))

(event EventOnStopDragging
  (bind _lightcannel (Timeline|LightTime Reverse)
    (:Update
      (Rendering|Material|SetScalarParameterValueonMaterials (Variables|Default|GetSM_Drag) "Time" _lightcannel))
    (:Finished
      (if (>= _lightcannel 5.8)
        (Rendering|SetVisibility (Variables|Default|GetSM_Stick_Active) true false)
        (Variables|Default|SetCanOpen true)))))

(event EventOnStartDragging
  (if (Variables|Default|GetCanDrag)
    (bind _lightcannel (Timeline|LightTime Play)
      (:Update
        (Rendering|Material|SetScalarParameterValueonMaterials (Variables|Default|GetSM_Drag) "Time" _lightcannel))
      (:Finished
        (if (>= _lightcannel 5.8)
          (Rendering|SetVisibility (Variables|Default|GetSM_Stick_Active) true false)
          (Variables|Default|SetCanOpen true))))))

(fn ConstructionScript)