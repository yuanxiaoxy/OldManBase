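; BP_BossCable is the boss-stage cable that tracks whether the player is on it and handles the ending transition.
; Entering stores the movement direction, flags the player as present and tells the Recevier that the player is safe.
; Exiting clears the flag and, if the Recevier is over, has AnimationBall play a UI video.
; AnimationBall's completion event then opens the GameStart level.
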(event Custom|PlayCompelete
  (Game|OpenLevel(byName) "GameStart"))

(event EventBeginPlay
  (|CallParentFunction) ; 此节点被禁用，将不会被调用。\n从引脚连出引线来编译功能。
)

(event Collision|EventActorBeginOverlap
  (params (OtherActor :type Actor%20Object%20Reference))
  (|CallParentFunction OtherActor) ; 此节点被禁用，将不会被调用。\n从引脚连出引线来编译功能。
)

(event EventTick
  (params (DeltaSeconds :type Float%20%28single-precision%29))
  (|CallParentFunction DeltaSeconds))

(event EventCharacterExitCable
  (params (CableMoveForward :type Boolean))
  (Variables|Default|SetMoveForward CableMoveForward)
  (Variables|Default|SetHasPlayer false)
  (if (Variables|/Game/Boss/BP_BossLevelManager.BP_BossLevelManager_C|GetIsOver (Variables|Default|GetRecevier))
    (Class|OldManAnimationBall|PlayVideoinUI (Variables|Default|GetAnimationBall))
    (EventDispatchers|BindEventtoAnimationBallPlayCompelete (Variables|Default|GetAnimationBall) (delegate Custom|PlayCompelete))))

(event EventCharacterEnterCable
  (params (CableMoveForward :type Boolean))
  (Variables|Default|SetMoveForward CableMoveForward)
  (Variables|Default|SetHasPlayer true)
  (Default|PlayerinSafe (Variables|Default|GetRecevier)))

(fn ConstructionScript
  (|CallParentFunction))