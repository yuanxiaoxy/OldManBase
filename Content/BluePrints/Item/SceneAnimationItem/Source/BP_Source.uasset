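; BP_Source is a scene animation actor that travels along a target spline in triggered steps.
; It snaps to its starting spline point, then each MoveToNextPoint call advances the index by two, restarts a Niagara effect and destroys the actor once past the last point.
; Tick moves it by spline distance using a per-index speed and runs until the target is reached, then disables itself.
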(event Custom|MoveToNextPoint
  (Math|Integer|IncrementInt (Variables|Default|GetIndex)
    (:%20%20
      (Math|Integer|IncrementInt (Variables|Default|GetIndex)
        (:%20%20
          (if (>= (Variables|Default|GetIndex) (Variables|Default|GetPointsCount))
            (Actor|DestroyActor)
            (else
              (Niagara|ReinitializeSystem (Variables|Default|GetNS_JS_JL000))
              (Variables|Default|SetTargetDistance (Spline|GetDistanceAlongSplineatSplinePoint (Variables|Default|GetSplineComponent) (Variables|Default|GetIndex)))
              (Actor|Tick|SetActorTickEnabled true)
              (Variables|Default|SetIsMoving true))))))))

(event EventBeginPlay
  (Variables|Default|SetSplineComponent (Variables|/Game/BluePrints/Item/SceneAnimationItem/BP_ItemSpline.BP_ItemSpline_C|GetSpline (Variables|Default|GetTargetSpline)))
  (Transformation|SetActorLocation (Spline|GetLocationatSplinePoint (Variables|Default|GetSplineComponent) (Variables|Default|GetIndex) "World") false false)
  (Variables|Default|SetCurrentDistance (Spline|GetDistanceAlongSplineatSplinePoint (Variables|Default|GetSplineComponent) (Variables|Default|GetIndex)))
  (Variables|Default|SetPointsCount (Spline|GetNumberOfSplinePoints (Variables|Default|GetSplineComponent))))

(event EventTick
  (params (DeltaSeconds :type Float%20%28single-precision%29))
  (if (Variables|Default|GetIsMoving)
    (Variables|Default|SetCurrentDistance (+ (Variables|Default|GetCurrentDistance) (* DeltaSeconds (Utilities|Array|Get(acopy) (Variables|Default|GetMoveSpeed) (Variables|Default|GetIndex)))))
    (if (>= (Variables|Default|GetCurrentDistance) (Variables|Default|GetTargetDistance))
      (Variables|Default|SetCurrentDistance (Variables|Default|GetTargetDistance))
      (Variables|Default|SetIsMoving false))
    (Transformation|SetActorLocation (Spline|GetLocationatDistanceAlongSpline (Variables|Default|GetSplineComponent) (Variables|Default|GetCurrentDistance) "World") false false)
    (if (not (Variables|Default|GetIsMoving))
      (Actor|Tick|SetActorTickEnabled false))))

(fn ConstructionScript)