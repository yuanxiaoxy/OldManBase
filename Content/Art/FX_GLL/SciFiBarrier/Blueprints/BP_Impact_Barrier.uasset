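; Sci-fi barrier Blueprint that shows impact effects on its mesh where physics hits exceed a force threshold.
; Construction creates a dynamic material instance from the barrier material.
; Each strong hit takes the first idle of three timelines, writes the hit location to that slot's material parameter, and animates radius and intensity, allowing three overlapping impacts and ignoring further hits.
; An optional curve overrides the timelines' radius track at BeginPlay.
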(event OnComponentHit(StaticMeshComponent)
  (params (HitComponent :type Primitive%20Component%20Object%20Reference) (OtherActor :type Actor%20Object%20Reference) (OtherComp :type Primitive%20Component%20Object%20Reference) (NormalImpulse :type Vector :default "0, 0, 0") (Hit :type Hit%20Result%20Structure%20%28by%20ref%29))
  (bind _location (Collision|BreakHitResult Hit))
  (bind _returnvalue (Math|Conversions|ToLinearColor(Vector) _location))
  (if (> (Math|Vector|VectorLengthSquared NormalImpulse) (Math|Float|Square (Variables|Barrier|GetHitThreshold)))
    (if (not (Audio|Components|Audio|IsPlaying (Variables|Default|GetImpact1)))
      (Rendering|Material|SetVectorParameterValue (Variables|Barrier|GetDyMat) "Impact1Position" _returnvalue :!class /Script/Engine.MaterialInstanceDynamic)
      (Components|Timeline|PlayfromStart (Variables|Default|GetImpact1))
      (elif (not (Audio|Components|Audio|IsPlaying (Variables|Default|GetImpact2)))
        (Rendering|Material|SetVectorParameterValue (Variables|Barrier|GetDyMat) "Impact2Position" _returnvalue :!class /Script/Engine.MaterialInstanceDynamic)
        (Components|Timeline|PlayfromStart (Variables|Default|GetImpact2))
        (elif (not (Audio|Components|Audio|IsPlaying (Variables|Default|GetImpact3)))
          (Rendering|Material|SetVectorParameterValue (Variables|Barrier|GetDyMat) "Impact3Position" _returnvalue :!class /Script/Engine.MaterialInstanceDynamic)
          (Components|Timeline|PlayfromStart (Variables|Default|GetImpact3)))))))

(event EventBeginPlay
  (bind _impactcurve (Variables|Barrier|GetImpactCurve)
    (:then
      (Class|TimelineComponent|SetFloatCurve (Variables|Default|GetImpact3) _impactcurve "Radius"))
    (:else)))

(fn ConstructionScript
  (bind _staticmeshcomponent (Variables|Debug|GetStaticMeshComponent))
  (Rendering|Material|SetMaterial _staticmeshcomponent 0 (Variables|Barrier|GetBarrierMaterial))
  (bind _returnvalue (Rendering|Material|CreateDynamicMaterialInstance _staticmeshcomponent 0 (Variables|Barrier|GetBarrierMaterial) "None" :!class /Script/Engine.PrimitiveComponent))
  (Variables|Barrier|SetDyMat _returnvalue))