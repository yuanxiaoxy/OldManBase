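; Boss head actor that flashes highlights on its chin, eyebrows and ears.
; Each blink event enables custom depth with a stencil value on that part's meshes, runs the post-process manager's animation for six times Duration, then clears both.
; Ear-complete events fade post-process out and clear a highlight after a short timer, though the right-ear one clears the right eyebrow instead of the ear.
; SetChinHeighLight is an empty stub.
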(event Custom|SetAllFalse
  (CallFunction|SetChinLightFalse)
  (CallFunction|SetLeftEyebrowFalse)
  (CallFunction|SetLeftEarLightFalse)
  (CallFunction|SetRightEyebrowFalse)
  (CallFunction|SetRightEarLightFalse))

(event Custom|自定义事件
  (params (TimerId :type String))
  (CallFunction|SetLeftEarLightFalse))

(event Custom|SetRightEarLightTrue
  (bind _rightear (Variables|Default|GetRightEar))
  (bind _returnvalue (Actor|GetComponentbyClass _rightear "/Script/Engine.StaticMeshComponent"))
  (Rendering|SetRenderCustomDepth _returnvalue true)
  (Rendering|SetCustomDepthStencilValue _returnvalue 2))

(event Custom|SetRightEyebrowTrue
  (bind _righteyebrow (Variables|Default|GetRightEyebrow))
  (bind _returnvalue (Actor|GetComponentbyClass _righteyebrow "/Script/Engine.StaticMeshComponent"))
  (Rendering|SetRenderCustomDepth _returnvalue true)
  (Rendering|SetCustomDepthStencilValue _returnvalue 3))

(event Custom|SetLeftEyebrowTrue
  (bind _lefteyebrow (Variables|Default|GetLeftEyebrow))
  (bind _returnvalue (Actor|GetComponentbyClass _lefteyebrow "/Script/Engine.StaticMeshComponent"))
  (Rendering|SetRenderCustomDepth _returnvalue true)
  (Rendering|SetCustomDepthStencilValue _returnvalue 3))

(event Custom|SetLeftEyebrowFalse
  (Rendering|SetRenderCustomDepth (Actor|GetComponentbyClass (Variables|Default|GetLeftEyebrow) "/Script/Engine.StaticMeshComponent") false))

(event Custom|SetLeftEarLightTrue
  (bind _leftear (Variables|Default|GetLeftEar))
  (bind _returnvalue (Actor|GetComponentbyClass _leftear "/Script/Engine.StaticMeshComponent"))
  (Rendering|SetRenderCustomDepth _returnvalue true)
  (Rendering|SetCustomDepthStencilValue _returnvalue 2))

(event Custom|SetLeftEarLightFalse
  (Rendering|SetRenderCustomDepth (Actor|GetComponentbyClass (Variables|Default|GetLeftEar) "/Script/Engine.StaticMeshComponent") false))

(event Custom|CustomEvent
  (params (TimerId :type String))
  (CallFunction|SetRightEyebrowFalse))

(event Custom|SetRightEarLightFalse
  (Rendering|SetRenderCustomDepth (Actor|GetComponentbyClass (Variables|Default|GetRightEar) "/Script/Engine.StaticMeshComponent") false))

(event Custom|SetChinLightTrue
  (bind _shangbar (Variables|Default|GetShangBaR))
  (bind _chin (Variables|Default|GetChin))
  (bind _shangbal (Variables|Default|GetShangBaL))
  (bind _shangbamid (Variables|Default|GetShangBaMid))
  (bind _returnvalue (Actor|GetComponentbyClass _shangbar "/Script/Engine.StaticMeshComponent"))
  (bind _returnvalue_2 (Actor|GetComponentbyClass _chin "/Script/Engine.StaticMeshComponent"))
  (bind _returnvalue_3 (Actor|GetComponentbyClass _shangbal "/Script/Engine.StaticMeshComponent"))
  (bind _returnvalue_4 (Actor|GetComponentbyClass _shangbamid "/Script/Engine.StaticMeshComponent"))
  (Rendering|SetRenderCustomDepth _returnvalue true)
  (Rendering|SetCustomDepthStencilValue _returnvalue 3)
  (Rendering|SetRenderCustomDepth _returnvalue_2 true)
  (Rendering|SetCustomDepthStencilValue _returnvalue_2 3)
  (Rendering|SetRenderCustomDepth _returnvalue_3 true)
  (Rendering|SetCustomDepthStencilValue _returnvalue_3 3)
  (Rendering|SetRenderCustomDepth _returnvalue_4 true)
  (Rendering|SetCustomDepthStencilValue _returnvalue_4 3))

(event Custom|SetChinLightFalse
  (Rendering|SetRenderCustomDepth (Actor|GetComponentbyClass (Variables|Default|GetShangBaR) "/Script/Engine.StaticMeshComponent") false)
  (Rendering|SetRenderCustomDepth (Actor|GetComponentbyClass (Variables|Default|GetChin) "/Script/Engine.StaticMeshComponent") false)
  (Rendering|SetRenderCustomDepth (Actor|GetComponentbyClass (Variables|Default|GetShangBaL) "/Script/Engine.StaticMeshComponent") false)
  (Rendering|SetRenderCustomDepth (Actor|GetComponentbyClass (Variables|Default|GetShangBaMid) "/Script/Engine.StaticMeshComponent") false))

(event Custom|SetRightEyebrowFalse
  (Rendering|SetRenderCustomDepth (Actor|GetComponentbyClass (Variables|Default|GetRightEyebrow) "/Script/Engine.StaticMeshComponent") false))

(event EventBeginPlay)

(event Collision|EventActorBeginOverlap
  (params (OtherActor :type Actor%20Object%20Reference)))

(event EventRightEarCompelete
  (Class|PostProcessManager|Fade2None (Class|PostProcessManager|GetPostProcessManager))
  (Class|MonoManager|SetTimeout (Class|MonoManager|GetMonoManager) 0.5 (delegate Custom|CustomEvent)))

(event EventTick
  (params (DeltaSeconds :type Float%20%28single-precision%29)))

(event EventRightEyebrowBlinkinBP
  (CallFunction|SetRightEyebrowTrue)
  (Class|PostProcessManager|StartPostProcessAnim (Class|PostProcessManager|GetPostProcessManager))
  (Utilities|FlowControl|Delay (* (Variables|Default|GetDuration) 6.0))
  (Class|PostProcessManager|StopPostProcessAnim (Class|PostProcessManager|GetPostProcessManager))
  (CallFunction|SetRightEyebrowFalse))

(event EventLeftEarBlinkinBP
  (CallFunction|SetLeftEarLightTrue)
  (Class|PostProcessManager|StartPostProcessAnim (Class|PostProcessManager|GetPostProcessManager))
  (Utilities|FlowControl|Delay (* (Variables|Default|GetDuration) 6.0))
  (Class|PostProcessManager|StopPostProcessAnim (Class|PostProcessManager|GetPostProcessManager))
  (CallFunction|SetLeftEarLightFalse))

(event EventLeftEyebrowBlinkinBP
  (CallFunction|SetLeftEyebrowTrue)
  (Class|PostProcessManager|StartPostProcessAnim (Class|PostProcessManager|GetPostProcessManager))
  (Utilities|FlowControl|Delay (* (Variables|Default|GetDuration) 6.0))
  (Class|PostProcessManager|StopPostProcessAnim (Class|PostProcessManager|GetPostProcessManager))
  (CallFunction|SetLeftEyebrowFalse))

(event EventRightEarBlinkinBP
  (CallFunction|SetRightEarLightTrue)
  (Class|PostProcessManager|StartPostProcessAnim (Class|PostProcessManager|GetPostProcessManager))
  (Utilities|FlowControl|Delay (* (Variables|Default|GetDuration) 6.0))
  (Class|PostProcessManager|StopPostProcessAnim (Class|PostProcessManager|GetPostProcessManager))
  (CallFunction|SetRightEarLightFalse))

(event EventChinBlinkinBP
  (CallFunction|SetChinLightTrue)
  (Class|PostProcessManager|StartPostProcessAnim (Class|PostProcessManager|GetPostProcessManager))
  (Utilities|FlowControl|Delay (* (Variables|Default|GetDuration) 6.0))
  (Class|PostProcessManager|StopPostProcessAnim (Class|PostProcessManager|GetPostProcessManager))
  (CallFunction|SetChinLightFalse))

(event EventLeftEarCompelete
  (Class|PostProcessManager|Fade2None (Class|PostProcessManager|GetPostProcessManager))
  (Class|MonoManager|SetTimeout (Class|MonoManager|GetMonoManager) 0.5 (delegate Custom|自定义事件)))

(fn ConstructionScript)

(fn SetChinHeighLight)