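; BP_OldManBullet is a bullet actor that plays a fire effect when spawned and a boom effect on impact.
; Both effects go through the effect manager by ID, placed at the actor on BeginPlay and at the mesh component on hit.
; A mesh hit also destroys the Niagara component and the actor.
; An unconnected branch that spawns and triggers a BP_FS_MasterField for destructible objects never runs.
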(event OnComponentHit(MeshComponent)
  (params (HitComponent :type Primitive%20Component%20Object%20Reference) (OtherActor :type Actor%20Object%20Reference) (OtherComp :type Primitive%20Component%20Object%20Reference) (NormalImpulse :type Vector :default "0, 0, 0") (Hit :type Hit%20Result%20Structure%20%28by%20ref%29))
  (bind _meshcomponent (Variables|Default|GetMeshComponent))
  (Class|EffectManager|PlayEffectatLocation (Class|EffectManager|GetEffectManager) (Variables|Default|GetBoomEffectID) (Transformation|GetWorldLocation _meshcomponent) (Transformation|GetWorldRotation _meshcomponent))
  (Components|DestroyComponent (Variables|Default|GetNiagara))
  (Actor|DestroyActor))

(event EventBeginPlay
  (Class|EffectManager|PlayEffectatLocation (Class|EffectManager|GetEffectManager) (Variables|Default|GetFireEffect%20ID) (Transformation|GetActorLocation) (Transformation|GetActorRotation)))

(event Collision|EventActorBeginOverlap
  (params (OtherActor :type Actor%20Object%20Reference)))

(event EventTick
  (params (DeltaSeconds :type Float%20%28single-precision%29)))

(fn ConstructionScript)