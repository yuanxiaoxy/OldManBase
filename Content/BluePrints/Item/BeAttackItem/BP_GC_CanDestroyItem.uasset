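; BP_GC_CanDestroyItem is an attackable item built on a Geometry Collection, apparently an unfinished prototype for a destructible object.
; A debug T key enables gravity on the collection, and Tick prints a test message while gravity is on.
; Component hits check the other actor for the tag_DetcedItem tag, then only run a short delay.
; A print, delay and DestroyActor chain is disconnected and never runs.
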(event OnComponentHit(GeometryCollection)
  (params (HitComponent :type Primitive%20Component%20Object%20Reference) (OtherActor :type Actor%20Object%20Reference) (OtherComp :type Primitive%20Component%20Object%20Reference) (NormalImpulse :type Vector :default "0, 0, 0") (Hit :type Hit%20Result%20Structure%20%28by%20ref%29))
  (if (> (Utilities|Array|FindItem (Variables|/Script/Engine.Actor|GetTags OtherActor) "tag_DetcedItem") -1)
    (Utilities|FlowControl|Delay 0.2)))

(event EventBeginPlay)

(event Collision|EventActorBeginOverlap
  (params (OtherActor :type Actor%20Object%20Reference)))

(event EventTick
  (params (DeltaSeconds :type Float%20%28single-precision%29))
  (if (Class|PrimitiveComponent|IsGravityEnabled (Variables|Default|GetGeometryCollection))
    (Development|PrintString "Hello")))

(event Input|KeyboardEvents|DebugKeyT
  (params (Key :type Key%20Structure :default "None") (ActionValue :type Input%20Action%20Value%20Structure))
  (:Pressed
    (Physics|SetEnableGravity (Variables|Default|GetGeometryCollection) true)))

(fn ConstructionScript)