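; Boss-area screen flash actor that pulses the view red or green for a given duration via a post process volume.
; FlashRed and FlashGreen each start a named MonoManager interval that toggles saturation, contrast and gamma between a tint and neutral.
; A timeout then clears that interval and restores neutral grading.
; Both colors share the IsA toggle flag and the same volume.
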(event Custom|CustomEvent_1
  (if (Variables|Default|GetIsA)
    (Variables|Default|SetIsA false)
    (Utilities|Struct|SetmembersinPostProcessSettings (Variables|/Script/Engine.PostProcessVolume|GetSettings (Variables|Default|GetPost%20Process%20Volum)) (Math|Vector4|MakeVector4 0.8 1.0 0.8 1.0) (Math|Vector4|MakeVector4 0.8 1.0 0.8 1.0) (Math|Vector4|MakeVector4 0.5 1.0 0.6 1.0))
    (else
      (Variables|Default|SetIsA true)
      (Utilities|Struct|SetmembersinPostProcessSettings (Variables|/Script/Engine.PostProcessVolume|GetSettings (Variables|Default|GetPost%20Process%20Volum)) (Math|Vector4|MakeVector4 1.0 1.0 1.0 1.0) (Math|Vector4|MakeVector4 1.0 1.0 1.0 1.0) (Math|Vector4|MakeVector4 1.0 1.0 1.0 1.0)))))

(event Custom|CustomEvent_2
  (params (TimerId :type String))
  (Class|MonoManager|ClearTimer (Class|MonoManager|GetMonoManager) "GreenFlash")
  (Utilities|Struct|SetmembersinPostProcessSettings (Variables|/Script/Engine.PostProcessVolume|GetSettings (Variables|Default|GetPost%20Process%20Volum)) (Math|Vector4|MakeVector4 1.0 1.0 1.0 1.0) (Math|Vector4|MakeVector4 1.0 1.0 1.0 1.0) (Math|Vector4|MakeVector4 1.0 1.0 1.0 1.0)))

(event Custom|FlashRed
  (params (Time :type Float%20%28single-precision%29))
  (Class|MonoManager|SetIntervalSimplewithId (Class|MonoManager|GetMonoManager) 0.2 "RedFlash" (delegate Custom|Blink))
  (Class|MonoManager|SetTimeout (Class|MonoManager|GetMonoManager) Time (delegate Custom|complete)))

(event Custom|Blink
  (if (Variables|Default|GetIsA)
    (Variables|Default|SetIsA false)
    (Utilities|Struct|SetmembersinPostProcessSettings (Variables|/Script/Engine.PostProcessVolume|GetSettings (Variables|Default|GetPost%20Process%20Volum)) (Math|Vector4|MakeVector4 2.0 0.19 0.23 1.0) (Math|Vector4|MakeVector4 1.59 0.56 0.55 1.0) (Math|Vector4|MakeVector4 0.83 0.79 0.8 1.0))
    (else
      (Variables|Default|SetIsA true)
      (Utilities|Struct|SetmembersinPostProcessSettings (Variables|/Script/Engine.PostProcessVolume|GetSettings (Variables|Default|GetPost%20Process%20Volum)) (Math|Vector4|MakeVector4 1.0 1.0 1.0 1.0) (Math|Vector4|MakeVector4 1.0 1.0 1.0 1.0) (Math|Vector4|MakeVector4 1.0 1.0 1.0 1.0)))))

(event Custom|complete
  (params (TimerId :type String))
  (Class|MonoManager|ClearTimer (Class|MonoManager|GetMonoManager) "RedFlash")
  (Utilities|Struct|SetmembersinPostProcessSettings (Variables|/Script/Engine.PostProcessVolume|GetSettings (Variables|Default|GetPost%20Process%20Volum)) (Math|Vector4|MakeVector4 1.0 1.0 1.0 1.0) (Math|Vector4|MakeVector4 1.0 1.0 1.0 1.0) (Math|Vector4|MakeVector4 1.0 1.0 1.0 1.0)))

(event Custom|FlashGreen
  (params (Time :type Float%20%28single-precision%29))
  (Class|MonoManager|SetIntervalSimplewithId (Class|MonoManager|GetMonoManager) 0.2 "GreenFlash" (delegate Custom|CustomEvent_1))
  (Class|MonoManager|SetTimeout (Class|MonoManager|GetMonoManager) Time (delegate Custom|CustomEvent_2)))

(event EventBeginPlay)

(event EventTick
  (params (DeltaSeconds :type Float%20%28single-precision%29)))

(event Collision|EventActorBeginOverlap
  (params (OtherActor :type Actor%20Object%20Reference)))

(fn ConstructionScript)