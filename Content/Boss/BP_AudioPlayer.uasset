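; BP_AudioPlayer is a boss audio helper that plays sounds from an indexed SoundGroup by chance, either repeatedly or once.
; PlayRandomSoundGrounp starts a MonoManager interval timer whose callback rolls against the GaiLv probability each JianGeShiJian interval, then plays the selected sound ID through the AudioManager.
; PlaySoundGrounpOnce makes the same roll immediately.
; Both entry points clear the previous timer, and StopCur cancels it.
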(event Custom|PlaySoundGrounpOnce
  (params (index :type Integer))
  (Variables|Default|SetCurSound (Utilities|Array|Get(acopy) (Variables|Default|GetSoundGroup) index))
  (Class|MonoManager|ClearTimer (Class|MonoManager|GetMonoManager) (Variables|Default|GetCurInterval))
  (if (<= (Math|Random|RandomIntegerinRange 1 100) (* (Variables|Default|GetGaiLv) 1e+02))
    (Class|AudioManager|PlaySound (Class|AudioManager|GetAudioManager) (Utilities|Array|Get(acopy) (Variables|Default|GetSoundGroup) index) 0 "0, 0, 0" 0.0 0.0 1.0)))

(event Custom|playSound
  (params (TimerId :type String))
  (if (<= (Math|Random|RandomIntegerinRange 1 100) (* (Variables|Default|GetGaiLv) 1e+02))
    (Class|AudioManager|PlaySound (Class|AudioManager|GetAudioManager) (Utilities|Array|Get(acopy) (Variables|Default|GetSoundGroup) (stale Custom|PlayRandomSoundGrounp index)) 0 "0, 0, 0" 0.0 0.0 1.0)))

(event Custom|StopCur
  (Class|MonoManager|ClearTimer (Class|MonoManager|GetMonoManager) (Variables|Default|GetCurInterval)))

(event Custom|PlayRandomSoundGrounp
  (params (index :type Integer))
  (Variables|Default|SetCurSound (Utilities|Array|Get(acopy) (Variables|Default|GetSoundGroup) index))
  (Class|MonoManager|ClearTimer (Class|MonoManager|GetMonoManager) (Variables|Default|GetCurInterval))
  (bind _returnvalue (Class|MonoManager|SetInterval (Class|MonoManager|GetMonoManager) (Variables|Default|GetJianGeShiJian) (delegate Custom|playSound)))
  (Variables|Default|SetCurInterval _returnvalue))

(event EventBeginPlay)

(event Collision|EventActorBeginOverlap
  (params (OtherActor :type Actor%20Object%20Reference)))

(event EventTick
  (params (DeltaSeconds :type Float%20%28single-precision%29)))

(fn ConstructionScript)