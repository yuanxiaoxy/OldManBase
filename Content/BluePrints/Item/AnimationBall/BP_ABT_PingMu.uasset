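; BP_ABT_PingMu is an AnimationBall item actor, apparently a screen ("PingMu"), that plays a short media clip and then removes itself.
; On BeginPlay it opens the Kf source on MyPlayer and binds to the media opened and closed events.
; Once the media opens, a MonoManager timeout closes the player after a short fixed delay, and the closed event destroys the actor.
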(event Custom|自定义事件
  (params (TimerId :type String))
  (Media|MediaPlayer|Close (Variables|Default|GetMyPlayer) :!class /Script/MediaAssets.MediaPlayer))

(event Custom|123
  (params (OpenedUrl :type String))
  (Class|MonoManager|SetTimeout (Class|MonoManager|GetMonoManager) 2.0 (delegate Custom|自定义事件)))

(event Custom|自定义事件_0
  (Actor|DestroyActor))

(event EventBeginPlay
  (bind _myplayer (Variables|Default|GetMyPlayer))
  (Media|MediaPlayer|BindEventtoOnMediaOpened _myplayer (delegate Custom|123))
  (Media|MediaPlayer|OpenSource _myplayer "/Game/Movies/AnimationBallTest/kf.kf")
  (Media|MediaPlayer|BindEventtoOnMediaClosed (Variables|Default|GetMyPlayer) (delegate Custom|自定义事件_0)))

(event Collision|EventActorBeginOverlap
  (params (OtherActor :type Actor%20Object%20Reference)))

(event EventTick
  (params (DeltaSeconds :type Float%20%28single-precision%29)))

(fn ConstructionScript)