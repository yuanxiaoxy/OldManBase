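; Task that waits for the player to perform a left or right horizontal jump while an Old Man pop-up is shown.
; On start it opens the UI named by UIName additively and caches it as an OldManPopUpUIBase panel.
; Each tick it checks the cached player's move state and completes on either horizontal jump.
; On completion it calls FinishPlayerAction on the cached panel.
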(event EventOnStartTask
  (bind _returnvalue (Class|UIManager|ShowUIbyName (Class|UIManager|GetUIManager) (Variables|Default|GetUIName) 0 "Additive"))
  (bind _asold_man_pop_up_uibase (Utilities|Casting|CastToOldManPopUpUIBase _returnvalue))
  (Variables|Default|SetCachePanel _asold_man_pop_up_uibase))

(event EventOnTick
  (params (DeltaTime :type Float%20%28single-precision%29))
  (bind _returnvalue (Class|TaskCheckPlayerAction|GetCachedPlayer))
  (Utilities|IsValid _returnvalue
    (:Is%20Valid
      (if (Utilities|Enum|Equal(Enum) (Variables|/Script/OldMan.OldManCharacter|GetCurPlayerMoveState _returnvalue) "LeftHorizontalJump")
        (Class|TaskBase|CompleteTask)
        (elif (Utilities|Enum|Equal(Enum) "RightHorizontalJump" (Variables|/Script/OldMan.OldManCharacter|GetCurPlayerMoveState _returnvalue))
          (Class|TaskBase|CompleteTask))))))

(event EventOnCompleteTask
  (Class|OldManPopUpUIBase|FinishPlayerAction (Variables|Default|GetCachePanel)))