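; BP_SourceTrigger is a one-shot trigger actor that advances a referenced Source object along its points when the player reaches it.
; On overlap, it checks the other actor for the player tag returned by GetTagPlayer.
; If the Source is not already moving, it calls MoveToNextPoint and destroys itself; otherwise the trigger stays in place for a later overlap.
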(event EventBeginPlay)

(event Collision|EventActorBeginOverlap
  (params (OtherActor :type Actor%20Object%20Reference))
  (bind _returnvalue (Class|GlobalTagName|GetTagPlayer))
  (if (> (Utilities|Array|FindItem (Variables|/Script/Engine.Actor|GetTags OtherActor) _returnvalue) -1)
    (if (not (Variables|/Game/BluePrints/Item/SceneAnimationItem/Source/BP_Source.BP_Source_C|GetIsMoving (Variables|Default|GetSource)))
      (Default|MovetoNextPoint (Variables|Default|GetSource))
      (Actor|DestroyActor))))

(event EventTick
  (params (DeltaSeconds :type Float%20%28single-precision%29)))

(fn ConstructionScript)