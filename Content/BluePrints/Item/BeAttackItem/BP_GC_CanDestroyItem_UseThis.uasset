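; Destructible item Blueprint built on a Geometry Collection, apparently a work in progress with debug prints.
; On a component hit it prints a message and destroys itself if the other actor carries the detected-item tag, a branch the author notes as erroring for an unknown reason.
; A debug T key enables gravity on the collection, and Tick prints every frame while gravity is on.
; A delayed-destroy chain is left unconnected.
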(event OnComponentHit(GeometryCollection)
  (params (HitComponent :type Primitive%20Component%20Object%20Reference) (OtherActor :type Actor%20Object%20Reference) (OtherComp :type Primitive%20Component%20Object%20Reference) (NormalImpulse :type Vector :default "0, 0, 0") (Hit :type Hit%20Result%20Structure%20%28by%20ref%29))
  (Development|PrintString "hitted")
  ;[1 1 1] 这里的蓝图报错,具体原因未知
  (if (> (Utilities|Array|FindItem (Variables|/Script/Engine.Actor|GetTags OtherActor) "tag_DetcedItem") -1)
    (Actor|DestroyActor)))

(event EventBeginPlay)

(event Collision|EventActorBeginOverlap
  (params (OtherActor :type Actor%20Object%20Reference)))

(event EventTick
  (params (DeltaSeconds :type Float%20%28single-precision%29))
  (if (Class|PrimitiveComponent|IsGravityEnabled (Variables|Default|GetGeometryCollection))
    (Development|PrintString "Hello")))

(event Collision|EventHit
  (params (MyComp :type Primitive%20Component%20Object%20Reference) (Other :type Actor%20Object%20Reference) (OtherComp :type Primitive%20Component%20Object%20Reference) (bSelfMoved :type Boolean) (HitLocation :type Vector :default "0, 0, 0") (HitNormal :type Vector :default "0, 0, 0") (NormalImpulse :type Vector :default "0, 0, 0") (Hit :type Hit%20Result%20Structure%20%28by%20ref%29)))

(event Input|KeyboardEvents|DebugKeyT
  (params (Key :type Key%20Structure :default "None") (ActionValue :type Input%20Action%20Value%20Structure))
  (:Pressed
    (Physics|SetEnableGravity (Variables|Default|GetGeometryCollection) true)))

(fn ConstructionScript)