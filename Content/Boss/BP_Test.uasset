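; BP_Test is a debug Blueprint in the Boss folder that drives the facial parts of a TestTarget.
; On Tick, a set Iscom flag activates all of the target's parts once and then clears itself.
; Otherwise it closes any open left eyebrow, chin or right eyebrow every frame, and it prints the chin's open state while that is true.
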(event EventBeginPlay)

(event Collision|EventActorBeginOverlap
  (params (OtherActor :type Actor%20Object%20Reference)))

(event EventTick
  (params (DeltaSeconds :type Float%20%28single-precision%29))
  (bind _testtarget (Variables|Default|GetTestTarget))
  (bind _testtarget_2 (Variables|Default|GetTestTarget))
  (bind _ischinopen (Variables|/Script/OldMan.OldManBossHead|GetIsChinOpen _testtarget_2))
  (if _ischinopen
    (Development|PrintString (Utilities|String|ToString(Boolean) _ischinopen)))
  (if (Variables|Default|Getiscom)
    (Class|OldManBossHead|SetAllPartActive (Variables|Default|GetTestTarget) true)
    (Variables|Default|Setiscom false)
    (else
      (if (Variables|/Script/OldMan.OldManBossHead|GetIsLeftEyebrowOpen _testtarget_2)
        (Class|OldManBossHead|LeftEyebrowClose _testtarget))
      (if _ischinopen
        (Class|OldManBossHead|ChinClose _testtarget))
      (if (Variables|/Script/OldMan.OldManBossHead|GetIsRightEyebrowOpen _testtarget_2)
        (Class|OldManBossHead|RightEyebrowClose _testtarget)))))

(fn ConstructionScript)