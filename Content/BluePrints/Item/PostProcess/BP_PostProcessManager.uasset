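; Post-process manager that controls the strength of an outline effect through a material's LightStrength parameter.
; On BeginPlay it creates a dynamic instance of M_OutLine_Inst and sets it as the PostProcess component's blendable.
; Events start or stop a timeline animation, set the strength directly, snap it to a bright shine, or run a fade timeline.
; Shine and Fade2None change only the material, leaving the cached LightStrength variable untouched.
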(event Custom|Shine
  (Rendering|Material|SetScalarParameterValue (Variables|Default|GetMaterialIns) "LightStrength" 15.0 :!class /Script/Engine.MaterialInstanceDynamic))

(event EventSetLightStrength
  (params (Value :type Float%20%28single-precision%29))
  (Rendering|Material|SetScalarParameterValue (Variables|Default|GetMaterialIns) "LightStrength" Value :!class /Script/Engine.MaterialInstanceDynamic)
  (Variables|Default|SetLightStrength Value))

(event EventFade2None
  (bind _新建轨道_0 (Timeline|Fade Play)
    (:Update
      (Rendering|Material|SetScalarParameterValue (Variables|Default|GetMaterialIns) "LightStrength" (* _新建轨道_0 15.0) :!class /Script/Engine.MaterialInstanceDynamic))))

(event EventStartPostProcessAnim
  (bind _outlineanim (Timeline|OutLineAnim PlayFromStart)
    (:Update
      (Rendering|Material|SetScalarParameterValue (Variables|Default|GetMaterialIns) "LightStrength" (* _outlineanim 15.0) :!class /Script/Engine.MaterialInstanceDynamic)
      (Variables|Default|SetLightStrength (* _outlineanim 15.0)))))

(event EventStopPostProcessAnim
  (bind _outlineanim (Timeline|OutLineAnim Stop)
    (:Update
      (Rendering|Material|SetScalarParameterValue (Variables|Default|GetMaterialIns) "LightStrength" (* _outlineanim 15.0) :!class /Script/Engine.MaterialInstanceDynamic)
      (Variables|Default|SetLightStrength (* _outlineanim 15.0)))))

(event EventBeginPlay
  (bind _returnvalue (Rendering|Material|CreateDynamicMaterialInstance "/Game/Art/Material/M_OutLine/M_OutLine_Inst.M_OutLine_Inst" "None" "None" :!class /Script/Engine.KismetMaterialLibrary))
  (bind _output_get (Variables|Default|SetMaterialIns _returnvalue))
  (|SetBy-RefVar (Utilities|Struct|BreakPostProcessSettings (Variables|/Script/Engine.PostProcessComponent|GetSettings (Variables|Default|GetPostProcess))) (Utilities|Struct|MakeWeightedBlendables (Utilities|Array|MakeArray (Utilities|Struct|MakeWeightedBlendable 1.0 _output_get))))
  (bind _returnvalue_2 (Rendering|Material|GetScalarParameterValue (Variables|Default|GetMaterialIns) "LightStrength" :!class /Script/Engine.MaterialInstanceDynamic))
  (Variables|Default|SetLightStrength _returnvalue_2))

(fn ConstructionScript)