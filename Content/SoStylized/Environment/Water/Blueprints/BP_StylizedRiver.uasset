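; Stylized river actor that builds a water surface along an editable spline in the construction script.
; It picks a water mesh by tile resolution and fits evenly stretched spline mesh segments to the spline length, avoiding a squished last tile.
; Segment tangents are clamped to mesh length, and cross-section scale follows RiverWidth.
; Each segment gets a dynamic water material instance whose coordinate offset is its tile index.
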(fn ConstructionScript
  (bind _river_width (Variables|Default|GetRiver%20Width))
  (bind _returnvalue (/ _river_width 1e+03))
  (Variables|Default|SetMesh (Utilities|Select :Index (Variables|Default|GetIndividual%20Tile%20Resolution) :NewEnumerator0 "/Game/SoStylized/Environment/Water/Meshes/SM_WaterRiver01.SM_WaterRiver01" :NewEnumerator1 "/Game/SoStylized/Environment/Water/Meshes/SM_WaterRiver02.SM_WaterRiver02" :NewEnumerator2 "/Game/SoStylized/Environment/Water/Meshes/SM_WaterRiver04.SM_WaterRiver04" :NewEnumerator3 "/Game/SoStylized/Environment/Water/Meshes/SM_WaterRiver08.SM_WaterRiver08" :NewEnumerator4 "/Game/SoStylized/Environment/Water/Meshes/SM_WaterRiver16.SM_WaterRiver16" :NewEnumerator5 "/Game/SoStylized/Environment/Water/Meshes/SM_WaterRiver32.SM_WaterRiver32"))
  (Variables|Default|SetMesh%20LengthX (.x (+ (Math|Vector|VectorGetAbs (.min (StaticMesh|GetBoundingBox (Variables|Default|GetMesh)))) (Math|Vector|VectorGetAbs (.max (StaticMesh|GetBoundingBox (Variables|Default|GetMesh))))))) ; How long is our mesh. This is great because we could theoretically\nchange this out for other stuff if we wanted to repurpose this asset.
  (bind _output_get (Variables|Default|SetSpline%20Length (Spline|GetSplineLength (Variables|Default|GetSpline)))) ; The overall length of our spline. Good to store this as it\nwill be used for a few things.
  (Variables|Default|SetMesh%20Tiles (+ (Math|Float|Truncate (/ _output_get (Variables|Default|GetMesh%20LengthX))) 1)) ; How many meshes we want to actually\nspawn along our spline, based on the\nmesh and spline lengths.
  (Variables|Default|SetMesh%20Tile%20Length (/ (Variables|Default|GetSpline%20Length) (Variables|Default|GetMesh%20Tiles))) ; Now, if we just used the normal length of the mesh and\nspaced tiles out that way, our last mesh in the chain is\ngoing to be squished and glitchy until you stretch it out.\n\nThis can be kind of limiting and also looks kinda broken.\nBy scaling each mesh slightly we can distribute the\ntiles better.
  (for _index (range 0 (- (Variables|Default|GetMesh%20Tiles) 1)) ; Loop through each tile. We subtract once since\nloops begin at 0.
    (bind _returnvalue_2 (AddComponent|AddSplineMeshComponent false))
    (Components|StaticMesh|SetStaticMesh _returnvalue_2 (Variables|Default|GetMesh))
    (bind _returnvalue_3 (Rendering|Material|CreateDynamicMaterialInstance _returnvalue_2 0 (Variables|Default|GetWater%20Material) "None" :!class /Script/Engine.PrimitiveComponent))
    (Rendering|Material|SetScalarParameterValue _returnvalue_3 "River Coordinate OffsetX" (Math|Conversions|ToFloat(Integer) _index) :!class /Script/Engine.MaterialInstanceDynamic)
    (SplineMesh|SetStartandEnd _returnvalue_2 (Spline|GetLocationatDistanceAlongSpline (Variables|Default|GetSpline) (* _index (Variables|Default|GetMesh%20Tile%20Length)) "Local") (Math|Vector|ClampVectorSize (Spline|GetTangentatDistanceAlongSpline (Variables|Default|GetSpline) (* _index (Variables|Default|GetMesh%20Tile%20Length)) "Local") 0.0 (Variables|Default|GetMesh%20LengthX)) (Spline|GetLocationatDistanceAlongSpline (Variables|Default|GetSpline) (* (+ _index 1) (Variables|Default|GetMesh%20Tile%20Length)) "Local") (Math|Vector|ClampVectorSize (Spline|GetTangentatDistanceAlongSpline (Variables|Default|GetSpline) (* (+ _index 1) (Variables|Default|GetMesh%20Tile%20Length)) "Local") 0.0 (Variables|Default|GetMesh%20LengthX)) true :!class /Script/Engine.SplineMeshComponent)
    (SplineMesh|SetStartScale _returnvalue_2 (Math|Vector2D|MakeVector2D _returnvalue 1.0) true :!class /Script/Engine.SplineMeshComponent)
    (SplineMesh|SetEndScale _returnvalue_2 (Math|Vector2D|MakeVector2D _returnvalue 1.0) true :!class /Script/Engine.SplineMeshComponent)))