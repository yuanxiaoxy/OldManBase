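; BP_EnemyManagerAgent is an editable front end that configures the enemy manager singleton with level enemy data.
; On BeginPlay it copies pool size, enemy classes, approach-enemy tuning, ink settings, textures and per-enemy infos into the manager, then calls InitializeSingleton.
; When EnableDebug is set, the construction script calls RefreshDebug to draw the configured AdEnemy infos for preview.
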(event Custom|RefreshDebug
  (if (Variables|Default|GetbEnableDebug)
    (Class|AdEnemyManagerAgent|DrawAdEnemyDebug (Variables|Default|GetBP_EnemyInfos) -1.0)))

(event EventBeginPlay
  (bind _output_get (Variables|Default|SetEnemyManager (Class|OldManEnemyManager|GetEnemyManager)))
  (bind _enemymanager (CallFunction|InsertValuetoManager _output_get))
  (Class|OldManEnemyManager|InitializeSingleton _enemymanager))

(event Collision|EventActorBeginOverlap
  (params (OtherActor :type Actor%20Object%20Reference)))

(event EventTick
  (params (DeltaSeconds :type Float%20%28single-precision%29)))

(fn ConstructionScript
  (if (Variables|Default|GetbEnableDebug)
    (CallFunction|RefreshDebug)))

(fn InsertValuetoManager
  (params (Manager :type Old%20Man%20Enemy%20Manager%20Object%20Reference))
  (bind _enemymanager (Variables|Default|GetEnemyManager))
  (LocalVariables|SetOldManEnemyManager Manager)
  (|InsertSingleValue (LocalVariables|GetOldManEnemyManager))
  (CallFunction|InsertApEnemy (LocalVariables|GetOldManEnemyManager))
  (for _array_element (Variables|Default|GetBP_EnemyInfos)
    (Class|OldManEnemyManager|AddInfo _enemymanager _array_element))
  (Variables|/Script/OldManEnemy.OldManEnemyManager|SetInkTextures _enemymanager (Variables|Default|GetInkTextures))
  (Variables|/Script/OldManEnemy.OldManEnemyManager|SetMultiInkTextures _enemymanager (Variables|Default|GetMultiInkTextures))
  (return _enemymanager))

(fn InsertApEnemy
  (params (Manager :type Old%20Man%20Enemy%20Manager%20Object%20Reference))
  (Variables|/Script/OldManEnemy.OldManEnemyManager|SetMaxApproachEnemyCount Manager (Variables|Default|GetApEnemy_MaxCount))
  (Variables|/Script/OldManEnemy.OldManEnemyManager|SetApEnemyApproachSpeed Manager (Variables|Default|GetApEnemy_Speed))
  (Variables|/Script/OldManEnemy.OldManEnemyManager|SetApEnemyAttackDistance Manager (Variables|Default|GetApEnemy_Distance))
  (Variables|/Script/OldManEnemy.OldManEnemyManager|SetApproachEnemySpawnInterval Manager (Variables|Default|GetApEnemy_SpawnInterval))
  (Variables|/Script/OldManEnemy.OldManEnemyManager|SetApEnemyAttackDistance Manager (Variables|Default|GetApEnemy_AttackDistance))
  (Variables|/Script/OldManEnemy.OldManEnemyManager|SetFlashDistance Manager (Variables|Default|GetApEnemy_FlashDistance)))