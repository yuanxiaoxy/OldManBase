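; Left eyebrow part of a boss head that reacts to taking damage and reports it to BossHeadPart.
; Any damage calls the head's eyebrow-open function, then, if the left eyebrow is active, sets its state true and raises post-process light strength.
; After a short delay it fades the effect out and starts a MonoManager timeout whose callback sets the eyebrow state back to false.
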(event Custom|Event_OnTakeAnyDamage
  (params (DamagedActor :type Actor%20Object%20Reference) (Damage :type Float%20%28single-precision%29) (DamageType :type Damage%20Type%20Object%20Reference) (InstigatedBy :type Controller%20Object%20Reference) (DamageCauser :type Actor%20Object%20Reference))
  (Class|OldManBossHead|LeftEyebrowOpen (Variables|Default|GetBossHeadPart))
  (if (Variables|/Script/OldMan.OldManBossHead|GetIsLeftEyebrowActive (Variables|Default|GetBossHeadPart))
    (Default|SetLeftEyebrowTrue (Variables|Default|GetBossHeadPart))
    (Class|PostProcessManager|SetLightStrength (Class|PostProcessManager|GetPostProcessManager) 15.0)
    (Utilities|FlowControl|Delay 0.5)
    (Class|PostProcessManager|Fade2None (Class|PostProcessManager|GetPostProcessManager))
    (Class|MonoManager|SetTimeout (Class|MonoManager|GetMonoManager) 0.5 (delegate Custom|自定义事件))))

(event Custom|自定义事件
  (params (TimerId :type String))
  (Default|SetLeftEyebrowFalse (Variables|Default|GetBossHeadPart)))

(event EventBeginPlay
  (EventDispatchers|AssignOnTakeAnyDamage (delegate Custom|Event_OnTakeAnyDamage)))

(event Collision|EventActorBeginOverlap
  (params (OtherActor :type Actor%20Object%20Reference)))

(fn ConstructionScript)