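; Task Blueprint that shows a swipe guide popup (HuaDong) and waits for the player to start pulling a draggable item.
; On start it fires the key-input pull-unlock event through both EventManager trigger calls, then opens and caches the guide panel.
; Each tick it polls the cached player's InPullState and completes the task once true.
; On completion it calls FinishPlayerAction on the cached panel.
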(event EventOnStartTask
  (bind _returnvalue (Class|MyEventManager|GetEventManager))
  (bind _gameeventdata (Utilities|Struct|MakeGameEventData))
  (bind _returnvalue_2 (Class|GlobalEventName|GetKeyInputUnLockPull))
  (Class|MyEventManager|TriggerCppEventUniversal _returnvalue _returnvalue_2 _gameeventdata)
  (Class|MyEventManager|TriggerEvent _returnvalue _returnvalue_2 _gameeventdata)
  (bind _returnvalue_3 (Class|UIManager|ShowUIbyName (Class|UIManager|GetUIManager) "PopupPanel_Guide_HuaDong" 0 "Additive" -1))
  (bind _asold_man_pop_up_uibase (Utilities|Casting|CastToOldManPopUpUIBase _returnvalue_3))
  (Variables|Default|SetCachePanel _asold_man_pop_up_uibase))

(event EventOnTick
  (params (DeltaTime :type Float%20%28single-precision%29))
  (bind _returnvalue (Class|TaskCheckPlayerAction|GetCachedPlayer))
  (Utilities|IsValid _returnvalue
    (:Is%20Valid
      (if (Variables|/Script/OldMan.OldManCharacter|GetbInPullState _returnvalue)
        (Class|TaskBase|CompleteTask)
        (else
          (Development|PrintText "Wait"))))))

(event EventOnCompleteTask
  (Development|PrintText "Hello")
  (Class|OldManPopUpUIBase|FinishPlayerAction (Variables|Default|GetCachePanel)))