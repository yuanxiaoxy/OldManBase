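; BP_ActorVisibleArea is a trigger area that toggles the lights of a set of referenced actors when the player enters it.
; An IsOpen flag picks the direction: open areas switch the lights off at BeginPlay and on at overlap, while others switch them off at overlap.
; Overlapping actors are filtered by the player tag, and an IsOnce flag destroys the area after it fires.
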(event EventBeginPlay
  (if (Variables|Default|GetIsOpen)
    (Default|CloseActorLights (Variables|Default|GetActors))))

(event Collision|EventActorBeginOverlap
  (params (OtherActor :type Actor%20Object%20Reference))
  (bind _returnvalue (Class|GlobalTagName|GetTagPlayer))
  (if (> (Utilities|Array|FindItem (Variables|/Script/Engine.Actor|GetTags OtherActor) _returnvalue) -1)
    (if (Variables|Default|GetIsOpen)
      (Default|OpenActorLights (Variables|Default|GetActors))
      (else
        (Default|CloseActorLights (Variables|Default|GetActors))))
    (if (Variables|Default|GetIsOnce)
      (Actor|DestroyActor))))

(event EventTick
  (params (DeltaSeconds :type Float%20%28single-precision%29)))

(fn ConstructionScript)