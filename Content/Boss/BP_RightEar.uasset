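; BP_RightEar is a boss's draggable right ear that feeds drag progress into the boss head.
; Start and stop dragging events toggle the IsDraged flag and the actor's tick.
; While dragged, Tick checks that the target cable has a player and moves in the direction set by TargetForward, then sends a clamped, speed-scaled delta to BossHead.RightEarDragedAdd.
; Custom-depth highlight logic exists but is unreachable.
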(event EventBeginPlay)

(event Collision|EventActorBeginOverlap
  (params (OtherActor :type Actor%20Object%20Reference)))

(event EventTick
  (params (DeltaSeconds :type Float%20%28single-precision%29))
  (if (Variables|Default|GetTargetForward)
    (if (and (Variables|/Game/Boss/BP_BossCable.BP_BossCable_C|GetMoveForward (Variables|Default|GetTargetCable)) (and (Variables|Default|GetIsDraged) (Variables|/Game/Boss/BP_BossCable.BP_BossCable_C|GetHasPlayer (Variables|Default|GetTargetCable))))
      (Class|OldManBossHead|RightEarDragedAdd (Variables|Default|GetBossHead) (Math|Float|Clamp(Float) (* DeltaSeconds (Variables|Default|GetMoveSpeed))) :!label _label))
    (elif (and (not (Variables|/Game/Boss/BP_BossCable.BP_BossCable_C|GetMoveForward (Variables|Default|GetTargetCable))) (and (Variables|Default|GetIsDraged) (Variables|/Game/Boss/BP_BossCable.BP_BossCable_C|GetHasPlayer (Variables|Default|GetTargetCable))))
      (goto _label))))

(event EventOnStartDragging
  (Variables|Default|SetIsDraged true)
  (Actor|Tick|SetActorTickEnabled true))

(event EventOnStopDragging
  (Variables|Default|SetIsDraged false)
  (Actor|Tick|SetActorTickEnabled false))

(fn ConstructionScript)