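; BP_TriggerAudioEffectArea is a one-shot trigger area that changes the effects on a playing sound when the player enters it.
; OnEnterTrigger checks the entering actor for the player tag, then has the audio manager apply an effect preset row to the configured sound ID.
; It also starts a timed low-pass lerp on that sound toward a target cutoff, then destroys itself.
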(event EventBeginPlay)

(event Collision|EventActorBeginOverlap
  (params (OtherActor :type Actor%20Object%20Reference)))

(event EventTick
  (params (DeltaSeconds :type Float%20%28single-precision%29)))

(event EventOnEnterTrigger
  (params (OverlappedComponent :type Primitive%20Component%20Object%20Reference) (OtherActor :type Actor%20Object%20Reference) (OtherComp :type Primitive%20Component%20Object%20Reference) (OtherBodyIndex :type Integer) (bFromSweep :type Boolean) (SweepResult :type Hit%20Result%20Structure%20%28by%20ref%29))
  (bind _returnvalue (Class|AudioManager|GetAudioManager))
  (bind _audioid (Variables|Default|GetAudioID))
  (bind _returnvalue_2 (Class|GlobalTagName|GetTagPlayer))
  (if (> (Utilities|Array|FindItem (Variables|/Script/Engine.Actor|GetTags OtherActor) _returnvalue_2) -1)
    (Class|AudioManager|ApplyEffectPresetbySoundID _returnvalue _audioid (Variables|Default|GetAudioEffectID))
    (Class|AudioManager|StartSoundLowPassLerp _returnvalue _audioid (Variables|Default|GetTargetCutOff) (Variables|Default|GetDuration))
    (Actor|DestroyActor)))

(fn ConstructionScript)