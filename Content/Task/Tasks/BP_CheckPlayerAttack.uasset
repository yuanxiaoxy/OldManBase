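; Tutorial task that teaches the player to attack and completes once an attack input is detected.
; On start it plays a guide voice line, listens to game events, opens an additive click-guide popup and fires the event that unlocks attack input.
; A matching attack-input event completes the task, which plays a follow-up voice line and tells the cached popup the player action is finished.
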(event Custom|OnAttack
  (params (EventName :type Name%20%28by%20ref%29) (EventData :type Game%20Event%20Data%20Structure%20%28by%20ref%29))
  (bind _returnvalue (Class|GlobalEventName|GetKeyInputInputAttack))
  (if (== _returnvalue EventName)
    (Class|TaskBase|CompleteTask)))

(event EventOnStartTask
  (bind _returnvalue (Game|GetPlayerCharacter 0))
  (Class|AudioManager|PlayVoice (Class|AudioManager|GetAudioManager) _returnvalue "L1_CaoZuo2" _returnvalue -1.0 -1.0 1.0)
  (EventDispatchers|BindEventtoOnGameEvent (Class|MyEventManager|GetEventManager) (delegate Custom|OnAttack))
  (bind _returnvalue_2 (Class|UIManager|ShowUIbyName (Class|UIManager|GetUIManager) "PopupPanel_Guide_DianJi" 0 "Additive"))
  (bind _asold_man_pop_up_uibase (Utilities|Casting|CastToOldManPopUpUIBase _returnvalue_2))
  (Variables|Default|SetCachePanel _asold_man_pop_up_uibase)
  (bind _returnvalue_3 (Class|GlobalEventName|GetKeyInputUnLockAttack))
  (Class|MyEventManager|TriggerCppEventUniversal (Class|MyEventManager|GetEventManager) _returnvalue_3 (Utilities|Struct|MakeGameEventData)))

(event EventOnCompleteTask
  (bind _returnvalue (Game|GetPlayerCharacter 0))
  (Development|PrintText "Hello")
  (Class|AudioManager|PlayVoice (Class|AudioManager|GetAudioManager) _returnvalue "L1_CaoZuo3" _returnvalue -1.0 -1.0 1.0)
  (Class|OldManPopUpUIBase|FinishPlayerAction (Variables|Default|GetCachePanel)))