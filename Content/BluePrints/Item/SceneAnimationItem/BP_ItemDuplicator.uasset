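; Scene animation spawner that fills a spline path with staggered copies of a template moving item.
; On BeginPlay it starts the template moving, then a delayed loop spawns Number copies at the spline's first point, spaced by IntervalTime.
; Each copy inherits the template's movement, float, timing and transform settings, then starts moving.
; Meshes are picked randomly from ItemStaticMesh, falling back to the template's mesh when that list is empty.
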(event EventBeginPlay
  (Default|MoveItem (Variables|Default|GetItem))
  (Utilities|ForLoopwithDelayFirst 0 (- (Variables|Default|GetNumber) 1) (Variables|Default|GetIntervalTime)
    (:LoopBody
      (if (!= (Utilities|Array|Length (Variables|Default|GetItem_StaticMesh)) 0)
        (bind _result (Math|Integer|DecrementInt (Utilities|Array|Length (Variables|Default|GetItem_StaticMesh)))
          (:%20%20
            (Variables|Default|SetnowStaticMesh (Utilities|Array|Get(acopy) (Variables|Default|GetItem_StaticMesh) (Math|Random|RandomIntegerinRange 0 _result)))))
        (else
          (Variables|Default|SetnowStaticMesh (Variables|/Game/BluePrints/Item/SceneAnimationItem/BP_ItemDuplicated.BP_ItemDuplicated_C|GetItemMesh (Variables|Default|GetItem)))))
      (bind _returnvalue (Game|SpawnActorfromClass (Utilities|GetClass (Variables|Default|GetItem)) (Math|Conversions|ToTransform(Vector) (Spline|GetLocationatSplinePoint (Variables|/Game/BluePrints/Item/SceneAnimationItem/BP_ItemSpline.BP_ItemSpline_C|GetSpline (Variables|/Game/BluePrints/Item/SceneAnimationItem/BP_ItemDuplicated.BP_ItemDuplicated_C|GetSplineToFollow (Variables|Default|GetItem))) 0 "World")) "Undefined" "MultiplyWithRoot" 0 0))
      (Variables|/Game/BluePrints/Item/SceneAnimationItem/BP_ItemDuplicated.BP_ItemDuplicated_C|SetSplineToFollow _returnvalue (Variables|/Game/BluePrints/Item/SceneAnimationItem/BP_ItemDuplicated.BP_ItemDuplicated_C|GetSplineToFollow (Variables|Default|GetItem)))
      (Variables|/Game/BluePrints/Item/SceneAnimationItem/BP_ItemDuplicated.BP_ItemDuplicated_C|SetItemMesh _returnvalue (Variables|/Game/BluePrints/Item/SceneAnimationItem/BP_ItemDuplicated.BP_ItemDuplicated_C|GetItemMesh (Variables|Default|GetItem)))
      (Variables|/Game/BluePrints/Item/SceneAnimationItem/BP_ItemDuplicated.BP_ItemDuplicated_C|SetFloatRate _returnvalue (Variables|/Game/BluePrints/Item/SceneAnimationItem/BP_ItemDuplicated.BP_ItemDuplicated_C|GetFloatRate (Variables|Default|GetItem)))
      (Variables|/Game/BluePrints/Item/SceneAnimationItem/BP_ItemDuplicated.BP_ItemDuplicated_C|SetFloatExtremum _returnvalue (Variables|/Game/BluePrints/Item/SceneAnimationItem/BP_ItemDuplicated.BP_ItemDuplicated_C|GetFloatExtremum (Variables|Default|GetItem)))
      (Variables|/Game/BluePrints/Item/SceneAnimationItem/BP_ItemDuplicated.BP_ItemDuplicated_C|SetLoop _returnvalue (Variables|/Game/BluePrints/Item/SceneAnimationItem/BP_ItemDuplicated.BP_ItemDuplicated_C|GetLoop (Variables|Default|GetItem)))
      (Variables|/Game/BluePrints/Item/SceneAnimationItem/BP_ItemDuplicated.BP_ItemDuplicated_C|SetReserveStart _returnvalue (Variables|/Game/BluePrints/Item/SceneAnimationItem/BP_ItemDuplicated.BP_ItemDuplicated_C|GetReserveStart (Variables|Default|GetItem)))
      (Variables|/Game/BluePrints/Item/SceneAnimationItem/BP_ItemDuplicated.BP_ItemDuplicated_C|SetIsFloat _returnvalue (Variables|/Game/BluePrints/Item/SceneAnimationItem/BP_ItemDuplicated.BP_ItemDuplicated_C|GetIsFloat (Variables|Default|GetItem)))
      (Class|TimelineComponent|SetFloatCurve (Variables|/Game/BluePrints/Item/SceneAnimationItem/BP_ItemDuplicated.BP_ItemDuplicated_C|Get时间轴 _returnvalue) (Variables|/Game/BluePrints/Item/SceneAnimationItem/BP_ItemDuplicated.BP_ItemDuplicated_C|GetFloatCurve (Variables|Default|GetItem)) "None")
      (Variables|/Game/BluePrints/Item/SceneAnimationItem/BP_ItemDuplicated.BP_ItemDuplicated_C|SetTime _returnvalue (Variables|/Game/BluePrints/Item/SceneAnimationItem/BP_ItemDuplicated.BP_ItemDuplicated_C|GetTime (Variables|Default|GetItem)))
      ;[1 1 1] 静态网格体
      (Variables|/Game/BluePrints/Item/SceneAnimationItem/BP_ItemDuplicated.BP_ItemDuplicated_C|SetItemMesh _returnvalue (Variables|Default|GetnowStaticMesh))
      (Components|StaticMesh|SetStaticMesh (Variables|/Game/BluePrints/Item/SceneAnimationItem/BP_ItemDuplicated.BP_ItemDuplicated_C|GetItem_0 _returnvalue) (Variables|Default|GetnowStaticMesh))
      (Transformation|SetRelativeTransform (Variables|/Game/BluePrints/Item/SceneAnimationItem/BP_ItemDuplicated.BP_ItemDuplicated_C|GetItem_0 _returnvalue) (Transformation|GetRelativeTransform (Variables|/Game/BluePrints/Item/SceneAnimationItem/BP_ItemDuplicated.BP_ItemDuplicated_C|GetItem_0 (Variables|Default|GetItem))) false false)
      (Transformation|SetActorScale3D _returnvalue (Transformation|GetActorScale3D (Variables|Default|GetItem)))
      (Default|MoveItem _returnvalue))))

(fn ConstructionScript)