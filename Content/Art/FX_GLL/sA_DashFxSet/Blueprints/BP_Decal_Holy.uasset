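; BP_Decal_Holy is a short-lived decal effect actor from the dash FX set that aligns itself to the surface beneath it.
; On BeginPlay it runs a short vertical Visibility trace around its location and rotates the actor's Z axis to the hit normal.
; It then destroys itself after the Lifetime delay.
; A random-yaw step for the Decal component exists in the graph but is disconnected, so it never runs.
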(event EventBeginPlay
  (bind _returnvalue (Transformation|GetActorLocation))
  (bind _outhit (Collision|LineTraceByChannel (+ _returnvalue "0, 0,10.000000") (- _returnvalue "0, 0,10.000000") "TraceTypeQuery1" false 0 "None"))
  (Transformation|SetActorRotation (Math|Rotator|MakeRotfromZ (.Normal (Collision|BreakHitResult _outhit))))
  (Utilities|FlowControl|Delay (Variables|Default|GetLifetime))
  (Actor|DestroyActor))

(fn ConstructionScript)