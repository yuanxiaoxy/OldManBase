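; BP_Item is a scene animation actor that moves a configurable static mesh along a referenced spline with a floating height offset.
; MoveItem picks a looping or one-shot timeline, scales its rate by Time, and plays it forward or in reverse.
; Timeline updates map progress to spline distance, set world location and rotation, and add a repeating curve-driven Z bob.
; BeginPlay is empty and the delayed self-start is disconnected, so the file never calls MoveItem itself.
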(event Custom|MoveItem
  (bind _splinetofollow (Variables|Default|GetSplineToFollow))
  (bind _splinetofollow_2 (Variables|Default|GetSplineToFollow))
  (bind _spline (Variables|/Game/BluePrints/Item/SceneAnimationItem/OldMan_Spline/BP_ItemSpline.BP_ItemSpline_C|GetSpline _splinetofollow))
  (bind _spline_2 (Variables|/Game/BluePrints/Item/SceneAnimationItem/OldMan_Spline/BP_ItemSpline.BP_ItemSpline_C|GetSpline _splinetofollow_2))
  (if (Variables|Default|GetLoop)
    (Components|Timeline|SetPlayRate (Variables|Default|GetMoveTimeLineLoop) (/ 1.0 (Variables|Default|GetTime)))
    (if (Variables|Default|GetReserveStart)
      (bind _movetrack (Timeline|MoveTimeLineLoop ReverseFromEnd)
        (:Update
          (Transformation|SetActorLocationAndRotation (Math|Vector|MakeVector (.x (Spline|GetLocationatDistanceAlongSpline _spline_2 (Math|Float|Lerp 0.0 (Spline|GetSplineLength _spline_2) _movetrack) "World")) (.y (Spline|GetLocationatDistanceAlongSpline _spline_2 (Math|Float|Lerp 0.0 (Spline|GetSplineLength _spline_2) _movetrack) "World")) (+ (.z (Spline|GetLocationatDistanceAlongSpline _spline_2 (Math|Float|Lerp 0.0 (Spline|GetSplineLength _spline_2) _movetrack) "World")) (* (Variables|Default|GetFloatExtremum) (Math|Curves|GetFloatValue (Variables|Default|GetFloatCurve) (Math|Float|%(Float) (* _movetrack (Variables|Default|GetFloatRate)) 1.0))))) (Spline|GetRotationatDistanceAlongSpline _spline_2 (Math|Float|Lerp 0.0 (Spline|GetSplineLength _spline_2) _movetrack) "World"))))
      (else
        (Timeline|MoveTimeLineLoop PlayFromStart)))
    (else
      (Components|Timeline|SetPlayRate (Variables|Default|GetMoveTimeLine) (/ 1.0 (Variables|Default|GetTime)))
      (if (Variables|Default|GetReserveStart)
        (bind _movetrack_2 (Timeline|MoveTimeLine ReverseFromEnd)
          (:Update
            (Transformation|SetActorLocationAndRotation (Math|Vector|MakeVector (.x (Spline|GetLocationatDistanceAlongSpline _spline (Math|Float|Lerp 0.0 (Spline|GetSplineLength _spline) _movetrack_2) "World")) (.y (Spline|GetLocationatDistanceAlongSpline _spline (Math|Float|Lerp 0.0 (Spline|GetSplineLength _spline) _movetrack_2) "World")) (+ (.z (Spline|GetLocationatDistanceAlongSpline _spline (Math|Float|Lerp 0.0 (Spline|GetSplineLength _spline) _movetrack_2) "World")) (* (Variables|Default|GetFloatExtremum) (Math|Curves|GetFloatValue (Variables|Default|GetFloatCurve) (Math|Float|%(Float) (* _movetrack_2 (Variables|Default|GetFloatRate)) 1.0))))) (Spline|GetRotationatDistanceAlongSpline _spline (Math|Float|Lerp 0.0 (Spline|GetSplineLength _spline) _movetrack_2) "World"))))
        (else
          (Timeline|MoveTimeLine PlayFromStart))))))

(event EventBeginPlay)

(fn ConstructionScript
  (Components|StaticMesh|SetStaticMesh (Variables|Default|GetItem_0) (Variables|Default|GetItemMesh)))