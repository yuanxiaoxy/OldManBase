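; BP_Effect is a Blueprint from the Niagara magical portal FX folder that spawns a configurable Niagara system, either once or repeatedly.
; On BeginPlay it sets a timer by function name, with variable interval and looping, that fires the Effect event.
; Effect waits for a delay, then spawns the system at the Sphere component's world location plus an offset, using the configured rotation and scale.
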(event Custom|Effect
  (Utilities|FlowControl|Delay (Variables|Default|GetDelay))
  (Niagara|SpawnSystematLocation (Variables|Default|GetNiagara) (+ (Transformation|GetWorldLocation (Variables|Default|GetSphere)) (Variables|Default|GetLocation)) (Variables|Default|GetRotation) (Variables|Default|GetScale)))

(event EventBeginPlay
  (Utilities|Time|SetTimerbyFunctionName 0 "Effect" (Variables|Default|GetTime) (Variables|Default|GetLooping)))

(fn ConstructionScript)